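; Player character for a 2D boss rush: moves horizontally, charges a drill by spinning input, and launches along the aim direction.
; Timed distance checks validate spins, raising drill levels from a per-level data array; idle progress decays by timer, and dispatchers broadcast changes.
; Drilling disables gravity and enables head/body colliders to damage bosses, trigger map actions or rebound, then resets charge.
; PaperZD jumps, camera shake, time dilation and immunity blink provide feedback.
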(event OnHealthChanged(BP_HealthComponent)
  (params (NewHealth :type Float%20%28double-precision%29))
  (Damaging|HurtPlayerCharacter))

(event OnComponentBeginOverlap(DrillDetection_Body)
  (params (OverlappedComponent :type Primitive%20Component%20Object%20Reference) (OtherActor :type Actor%20Object%20Reference) (OtherComp :type Primitive%20Component%20Object%20Reference) (OtherBodyIndex :type Integer) (bFromSweep :type Boolean) (SweepResult :type Hit%20Result%20Structure%20%28by%20ref%29))
  (if (Variables|Drill|GetisDrilling)
    (Utilities|Casting|CastToBP_BasicMap OtherActor)
    (Development|PrintString "Collided to end drill on body" false)
    (Variables|/Script/Engine.CharacterMovementComponent|SetGravityScale (Variables|Character|GetCharacterMovement) 1.0)
    (Movement|RebounceCharacter "(X=0.000000,Y=150.000000)" false true)
    (Utilities|FlowControl|Delay 0.1)
    (Drill|EndDrilling false)))

(event Custom|EndDrillingForTimer
  (Drill|EndDrilling false))

(event Custom|SearchForActorsAtTheDrillCollider
  (bind _drilldetection_head (Variables|Default|GetDrillDetection_Head))
  (bind _overlappingactors (Collision|GetOverlappingActors _drilldetection_head "/Game/Blueprints/Map/BP_BasicMap.BP_BasicMap_C" :!class /Script/Engine.PrimitiveComponent))
  (bind _overlappingactors_2 (Collision|GetOverlappingActors _drilldetection_head "/Game/Blueprints/Bosses/BP_Boss.BP_Boss_C" :!class /Script/Engine.PrimitiveComponent))
  (bind _output (Utilities|Array|Get(acopy) _overlappingactors))
  (bind _output_2 (Utilities|Array|Get(acopy) _overlappingactors_2))
  (bind _asbp_boss (Utilities|Casting|CastToBP_Boss _output_2))
  (if (Variables|Drill|GetisDrilling)
    (Utilities|FlowControl|DoOnce false :!label _label
      (:Completed
        (Utilities|IsValid _asbp_boss
          (:Is%20Valid
            (CallFunction|SpawnVFXonDrillTip "/Game/Art/VFX/Animations/PC_Impact_VFX.PC_Impact_VFX" 1.4e+02)
            (Utilities|Time|ClearandInvalidateTimerbyHandle (Variables|Drill|GetEndDrillingTimer))
            (Variables|/Script/Engine.CharacterMovementComponent|SetGravityScale (Variables|Character|GetCharacterMovement) 1.0)
            (Damaging|DamageEnemy _asbp_boss)
            (Utilities|FlowControl|Delay 0.3)
            (Drill|EndDrilling true)
            (goto _label Reset))
          (:Is%20Not%20Valid
            (Utilities|IsValid _output
              (:Is%20Valid
                (bind _asbp_basic_map (Utilities|Casting|CastToBP_BasicMap _output)
                  (:then
                    (Default|CallPlayerActionwhenDrilling _asbp_basic_map self)
                    (goto _label Reset))
                  (:CastFailed
                    (goto _label Reset))))
              (:Is%20Not%20Valid
                (goto _label Reset)))))))))

(event Input|EnhancedActionEvents|EnhancedInputActionIA_Move
  (params (ActionValue :type Vector%202D%20Structure) (ElapsedSeconds :type Float%20%28double-precision%29) (TriggeredSeconds :type Float%20%28double-precision%29) (InputAction :type Input%20Action%20Object%20Reference :default "/Game/GameConfiguration/Input/Actions/IA_Move.IA_Move"))
  (:Triggered
    (bind _output_get (Variables|Movement|SetAimingDirection ActionValue))
    (if (not (Variables|Drill|GetisDrilling))
      (Finger|FingerAppearsandUpdatesPosition)
      (Pawn|Input|AddMovementInput (Class|KismetMathLibrary|VectorForward) (.x _output_get) false)
      (CallFunction|CalculateRotationOftheSprite)
      (Variables|Movement|SetisMoving true)))
  (:Canceled
    (Variables|Movement|SetAimingDirection "(X=0.000000,Y=1.000000)" :!label _label)
    (Variables|RotationInfo|SetisRotating false)
    (Variables|Movement|SetisMoving false)
    (Finger|LaunchTimertoHideFinger))
  (:Completed
    (goto _label)))

(event Input|EnhancedActionEvents|EnhancedInputActionIA_Drill
  (params (ActionValue :type Boolean) (ElapsedSeconds :type Float%20%28double-precision%29) (TriggeredSeconds :type Float%20%28double-precision%29) (InputAction :type Input%20Action%20Object%20Reference :default "/Game/GameConfiguration/Input/Actions/IA_Drill.IA_Drill"))
  (:Started
    (if (and (Variables|Drill|GetcanPlayerDrill) (not (Variables|Drill|GetisDrilling)))
      (Utilities|Time|ClearandInvalidateTimerbyHandle (Variables|Spin|GetDecereaseTimerEvent))
      (Variables|Drill|SetcanPlayerDrill false)
      (Variables|Spin|SetIsSpinning false)
      (Variables|Data|SetCurrentUsedDrillInformation (Utilities|Array|Get(acopy) (Variables|Data|GetSpinInformationLevels) (Variables|Drill|GetCurrentDrillLevel)))
      (Drill|DrillCollisionsEnabling true)
      (Drill|DrillIntoADirection (Variables|Movement|GetAimingDirection))
      (bind _returnvalue (Utilities|Time|SetTimerbyEvent (delegate Custom|EndDrillingForTimer) (.amountoftimedrilling (Variables|Data|GetCurrentUsedDrillInformation))))
      (Variables|Drill|SetEndDrillingTimer _returnvalue))))

(event Input|EnhancedActionEvents|EnhancedInputActionIA_Spin
  (params (ActionValue :type Vector%202D%20Structure) (ElapsedSeconds :type Float%20%28double-precision%29) (TriggeredSeconds :type Float%20%28double-precision%29) (InputAction :type Input%20Action%20Object%20Reference :default "/Game/GameConfiguration/Input/Actions/IA_Spin.IA_Spin"))
  (:Triggered
    (if (not (Variables|Drill|GetisDrilling))
      (if (Variables|Spin|GetIsSpinning)
        (Development|PrintString (Utilities|String|Append "Spinningvalues:   " (Utilities|String|ToString(Vector2d) ActionValue) "  --  This current time :   " (Utilities|String|ToString(Float) ElapsedSeconds)) false)
        (bind _isvalidspin (Spin|IsAvalidSpin (Utilities|Struct|MakeSTR_LastCorrectSpinData ActionValue ElapsedSeconds)))
        (if _isvalidspin
          (Variables|Spin|SetLastCorrectSpinningTime ElapsedSeconds)
          (Spin|IncrementCurrentSpins)
          (Utilities|Time|ClearandInvalidateTimerbyHandle (Variables|Spin|GetDecereaseTimerEvent))
          (elif (>= ElapsedSeconds (+ (Variables|Spin|GetLastCorrectSpinningTime) (.timewithoutthenextcorrecltinput (Utilities|Array|Get(acopy) (Variables|Data|GetSpinInformationLevels) (Variables|Drill|GetCurrentDrillLevel)))))
            (Spin|CreateInputRemoverTimer 0.0)))
        (else
          (Variables|Spin|SetLastReadedSpin (Utilities|Struct|MakeSTR_LastCorrectSpinData ActionValue ElapsedSeconds) :!label _label)
          (Variables|Spin|SetIsSpinning true)
          (Variables|Spin|SetLastCorrectSpinningTime ElapsedSeconds)))))
  (:Started
    (if (not (Variables|Drill|GetisDrilling))
      (goto _label)))
  (:Canceled
    (if (not (Variables|Drill|GetisDrilling)) :!label _label_2
      (Variables|Spin|SetIsSpinning false)
      (Development|PrintString "Stopped Spining" false)
      (Spin|CreateInputRemoverTimer (.timewithoutthenextcorrecltinput (Utilities|Array|Get(acopy) (Variables|Data|GetSpinInformationLevels) (Variables|Drill|GetCurrentDrillLevel))))))
  (:Completed
    (goto _label_2)))

(event EventBeginPlay
  (Utilities|FlowControl|Sequence
    (:then_0
      ;[1 1 1] Event Dispatchers to update the information
      (Default|CallChangeAmountOfLevelDrill (Variables|Drill|GetCurrentDrillLevel) false)
      (Default|CallChangeAmountOfCorrectInput 0 (.neededcorrectinputsforthenextlevel (Utilities|Array|Get(acopy) (Variables|Data|GetSpinInformationLevels) (Variables|Drill|GetCurrentDrillLevel))) true))
    (:then_1
      ;[1 1 1] Assign the input Mapping
      (bind _asplayer_controller (Utilities|Casting|CastToPlayerController (Pawn|GetController)))
      (Utilities|IsValid (PlayerController|LocalPlayerSubsystems|GetEnhancedInputLocalPlayerSubsystem _asplayer_controller)
        (:Is%20Valid
          (Input|AddMappingContext (PlayerController|LocalPlayerSubsystems|GetEnhancedInputLocalPlayerSubsystem _asplayer_controller) "/Game/GameConfiguration/Input/IMC_BossRushCharacterInput.IMC_BossRushCharacterInput" 0 "(bIgnoreAllPressedKeysUntilRelease=True,bForceImmediately=False,bNotifyUserSettings=False)"))))
    (:then_2
      (bind _returnvalue (Actor|GetActorOfClass "/Game/Blueprints/Camera/BP_Camera.BP_Camera_C"))
      (Utilities|IsValid _returnvalue
        (:Is%20Valid
          (Variables|Movement|SetBP_Camera _returnvalue))))
    (:then_3
      (bind _returnvalue_2 (Game|SpawnActorfromClass "/Game/Blueprints/BP_Finger.BP_Finger_C" (Transformation|GetActorTransform) "AlwaysSpawn" "OverrideRootScale" 0 0))
      (Variables|Finger|SetFingerReference _returnvalue_2)
      (Finger|FingerHides))))

(event Input|GamepadEvents|DebugKeyGamepadFaceButtonRight
  (params (Key :type Key%20Structure :default "None") (ActionValue :type Input%20Action%20Value%20Structure))
  (:Pressed
    (Damaging|HurtPlayerCharacter)))

(event Input|KeyboardEvents|DebugKeyH
  (params (Key :type Key%20Structure :default "None") (ActionValue :type Input%20Action%20Value%20Structure))
  (:Pressed
    (Damaging|HurtPlayerCharacter)))

(event Custom|SquashSprite
  (bind _sprite (Variables|Default|GetSprite))
  (bind _relativescale3d (Variables|/Script/Engine.SceneComponent|GetRelativeScale3D _sprite))
  (bind _zscalevalue (Timeline|SquashTimeline PlayFromStart)
    (:Update
      (Transformation|SetRelativeScale3D _sprite (Math|Vector|MakeVector (.x _relativescale3d) (.y _relativescale3d) _zscalevalue)))))

(event Custom|StopInmunityFeel
  (Utilities|FlowControl|Sequence
    (:then_0
      (bind _alpha (Timeline|BlinkInmunity Stop)
        (:Update
          (Sprite|SetSpriteColor (Variables|Default|GetSprite) (Utilities|Struct|MakeLinearColor 1.0 1.0 1.0 _alpha))
          (Sprite|SetSpriteColor (Variables|Default|GetConeDrill_Flipbook) (Utilities|Struct|MakeLinearColor 1.0 1.0 1.0 _alpha)))))
    (:then_1
      (Sprite|SetSpriteColor (Variables|Default|GetSprite) "(R=1.000000,G=1.000000,B=1.000000,A=1.000000)")
      (Sprite|SetSpriteColor (Variables|Default|GetConeDrill_Flipbook) "(R=1.000000,G=1.000000,B=1.000000,A=1.000000)"))))

(event Custom|StartInmunityFeel
  (bind _alpha (Timeline|BlinkInmunity PlayFromStart)
    (:Update
      (Sprite|SetSpriteColor (Variables|Default|GetSprite) (Utilities|Struct|MakeLinearColor 1.0 1.0 1.0 _alpha))
      (Sprite|SetSpriteColor (Variables|Default|GetConeDrill_Flipbook) (Utilities|Struct|MakeLinearColor 1.0 1.0 1.0 _alpha)))))

(fn ConstructionScript
  (Utilities|FlowControl|Sequence
    (:then_0
      (if (not (Class|KismetSystemLibrary|IsPackagedforDistribution))
        (Development|SetHiddeninGame (Variables|Default|GetCapsuleComponent) false false)))
    (:then_1
      (Movement|UpdateHeadCollider)
      (Variables|RotationInfo|SetPreviousRotationValue (.yaw (Transformation|GetActorRotation)))
      (Drill|DrillCollisionsEnabling false))))

(fn IncrementCurrentSpins
  (bind _result (Math|Integer|IncrementInt (Variables|Spin|GetCurrentCorrectInputsOfTheLevel))
    (:%20%20
      (if (> _result (.neededcorrectinputsforthenextlevel (Utilities|Array|Get(acopy) (Variables|Data|GetSpinInformationLevels) (Variables|Drill|GetCurrentDrillLevel))))
        (Variables|Spin|SetCurrentCorrectInputsOfTheLevel (Math|Integer|Clamp(Integer) (Variables|Spin|GetCurrentCorrectInputsOfTheLevel) 0 (.neededcorrectinputsforthenextlevel (Utilities|Array|Get(acopy) (Variables|Data|GetSpinInformationLevels) (Variables|Drill|GetCurrentDrillLevel)))))
        (if (== (Variables|Drill|GetCurrentDrillLevel) (- (Utilities|Array|Length (Variables|Data|GetSpinInformationLevels)) 1))
          (Development|PrintString "Maxed Amount of posible spins" false)
          (Default|CallMaxedLevelSpinsandInputs)
          (else
            (bind _output_get (Variables|Drill|SetCurrentDrillLevel (Math|Integer|Clamp(Integer) (+ (Variables|Drill|GetCurrentDrillLevel) 1) 0 (- (Utilities|Array|Length (Variables|Data|GetSpinInformationLevels)) 1))))
            (Variables|Spin|SetCurrentCorrectInputsOfTheLevel 0)
            (Development|PrintString (Utilities|String|Append "Moved to the next Spin Level:    " (Utilities|String|ToString(Integer) _output_get)) false)
            (Default|CallChangeAmountOfCorrectInput 0 0 true)
            (Default|CallChangeAmountOfLevelDrill (Variables|Drill|GetCurrentDrillLevel) false)
            (Movement|UpdateHeadCollider)))
        (else
          (Development|PrintString (Utilities|String|Append "Increment to Correct Input:    " (Utilities|String|ToString(Integer) _result)) false)
          (Default|CallChangeAmountOfCorrectInput (Variables|Spin|GetCurrentCorrectInputsOfTheLevel) (.neededcorrectinputsforthenextlevel (Utilities|Array|Get(acopy) (Variables|Data|GetSpinInformationLevels) (Variables|Drill|GetCurrentDrillLevel))) true))))))

(fn CreateInputRemoverTimer
  (params (DelayToStart :type Float%20%28double-precision%29))
  (if (not (Class|KismetSystemLibrary|TimerExistsHandle (Variables|Spin|GetDecereaseTimerEvent)))
    (Development|PrintString "Created new Decrement Timer" false)
    (bind _returnvalue (Utilities|Time|SetTimerbyEvent (EventDispatchers|CreateEvent :!event DecreaseCurrentSpinsbyTimer) (.ticktimetoreducecurrentspins (Utilities|Array|Get(acopy) (Variables|Data|GetSpinInformationLevels) (Variables|Drill|GetCurrentDrillLevel))) true false DelayToStart))
    (Variables|Spin|SetDecereaseTimerEvent _returnvalue)))

(fn DecreaseCurrentSpinsbyTimer
  (bind _spininformationlevels (Variables|Data|GetSpinInformationLevels))
  (bind _currentdrilllevel (Variables|Drill|GetCurrentDrillLevel))
  (bind _output (Utilities|Array|Get(acopy) _spininformationlevels _currentdrilllevel))
  (bind _output_get (Variables|Spin|SetCurrentCorrectInputsOfTheLevel (Math|Integer|Clamp(Integer) (- (Variables|Spin|GetCurrentCorrectInputsOfTheLevel) 1) 0 (.neededcorrectinputsforthenextlevel _output))))
  (Default|CallChangeAmountOfCorrectInput _output_get (.neededcorrectinputsforthenextlevel _output) false)
  (Development|PrintString (Utilities|String|Append "Removed Correct Input to:        " (Utilities|String|ToString(Integer) _output_get)) false)
  (if (== _output_get 0)
    (Utilities|Time|ClearandInvalidateTimerbyHandle (Variables|Spin|GetDecereaseTimerEvent))))

(fn IsAvalidSpin
  (params (NewSpin :type STR%20Last%20Correct%20Spin%20Data%20Structure))
  (bind _currentdrilllevel (Variables|Drill|GetCurrentDrillLevel))
  (bind _spininformationlevels (Variables|Data|GetSpinInformationLevels))
  (bind _output (Utilities|Array|Get(acopy) _spininformationlevels _currentdrilllevel))
  (LocalVariables|SetTimeToListenToTheNextInputLocal (.timetolistentothenextinput _output))
  (LocalVariables|SetMinDistanceLocal (.mindistancefromthelastcorrectinput _output))
  (LocalVariables|SetMaxDistanceLocal (.maxdistancefromthelastcorrectinput _output))
  (if (not (> (.time NewSpin) (+ (LocalVariables|GetTimeToListenToTheNextInputLocal) (.time (Variables|Spin|GetLastReadedSpin)))))
    (LocalVariables|SetIsvalidSpinLocal false)
    (Development|PrintString "Incorrect Time" false true "(R=1.000000,G=0.814895,B=0.000000,A=1.000000)")
    (Variables|Spin|SetLastReadedSpin (Utilities|Struct|MakeSTR_LastCorrectSpinData (.vectordirection NewSpin) (.time (Variables|Spin|GetLastReadedSpin)))) ; I want to have reads and not loose them because time precision
    (else
      (Development|PrintString (Utilities|String|Append "Distance from previous: " (Utilities|String|ToString(Float) (Math|Vector|Distance2D(Vector) (.vectordirection NewSpin) (.vectordirection (Variables|Spin|GetLastReadedSpin))))) false)
      (if (and (>= (Math|Vector|Distance2D(Vector) (.vectordirection NewSpin) (.vectordirection (Variables|Spin|GetLastReadedSpin))) (LocalVariables|GetMinDistanceLocal)) (<= (Math|Vector|Distance2D(Vector) (.vectordirection NewSpin) (.vectordirection (Variables|Spin|GetLastReadedSpin))) (LocalVariables|GetMaxDistanceLocal)))
        (LocalVariables|SetIsvalidSpinLocal true)
        (Development|PrintString "Correct Input" false true "(R=0.000000,G=1.000000,B=0.138889,A=1.000000)")
        (else
          (LocalVariables|SetIsvalidSpinLocal false)
          (Development|PrintString "Incorrect Input" false true "(R=1.000000,G=0.000000,B=0.113781,A=1.000000)")))
      (Variables|Spin|SetLastReadedSpin (Utilities|Struct|MakeSTR_LastCorrectSpinData (.vectordirection NewSpin) (.time NewSpin))) ; updating times because no matter the direction is ok or not, the read was in time
    ))
  (return (LocalVariables|GetIsvalidSpinLocal)))

(fn DrillCollisionsEnabling
  (params (EnableDrillCollisions :type Boolean))
  (if EnableDrillCollisions
    (Collision|SetCollisionEnabled (Variables|Default|GetDrillDetection_Head) "QueryOnly")
    (Collision|SetCollisionEnabled (Variables|Default|GetDrillDetection_Body) "QueryOnly")
    (else
      (Collision|SetCollisionEnabled (Variables|Default|GetDrillDetection_Head) "NoCollision")
      (Collision|SetCollisionEnabled (Variables|Default|GetDrillDetection_Body) "NoCollision"))))

(fn ConsumeAllSpinsforDrill
  (params (isFromDrilling :type Boolean))
  (bind _output_get (Variables|Drill|SetCurrentDrillLevel 0))
  (Default|CallChangeAmountOfLevelDrill _output_get isFromDrilling)
  (bind _output_get_2 (Variables|Spin|SetCurrentCorrectInputsOfTheLevel 0))
  (Default|CallChangeAmountOfCorrectInput _output_get_2 (.neededcorrectinputsforthenextlevel (Utilities|Array|Get(acopy) (Variables|Data|GetSpinInformationLevels) (Variables|Drill|GetCurrentDrillLevel))) isFromDrilling)
  (Movement|UpdateHeadCollider))

(fn DrillIntoADirection
  (params (DirectionToStartDrilling :type Vector%202D%20Structure))
  (bind _returnvalue (Math|Vector2D|MakeVector2D 0.0 1.0))
  (bind _returnvalue_2 (Math|Vector2D|Normalize2D DirectionToStartDrilling))
  (bind _returnvalue_3 (Math|Vector2D|DotProduct(2D) _returnvalue _returnvalue_2))
  (bind _returnvalue_4 (Math|Vector2D|Vector2DLength _returnvalue_2))
  (bind _returnvalue_5 (Math|Vector2D|Vector2DLength _returnvalue))
  (bind (_x _y) (Math|Vector2D|BreakVector2D _returnvalue_2))
  (bind _returnvalue_6 (* _returnvalue_5 _returnvalue_4))
  (bind _returnvalue_7 (/ _returnvalue_3 _returnvalue_6))
  (bind _returnvalue_8 (Class|KismetMathLibrary|DegAcos _returnvalue_7))
  (Finger|FingerHides)
  (Development|PrintString (Utilities|String|Append "Drill Direction:     " (Utilities|String|ToString(Vector2d) DirectionToStartDrilling)) false)
  (Variables|Drill|SetisDrilling true)
  (Class|PaperZDAnimInstance|JumptoNode (Variables|/Script/PaperZD.PaperZDAnimationComponent|GetAnimInstance (Variables|Default|GetAnimationComponent)) "Drill_Jump" "BasicStateMachine")
  (Variables|/Script/Engine.CharacterMovementComponent|SetGravityScale (Variables|Character|GetCharacterMovement) 0.0)
  (if (not (Class|KismetSystemLibrary|IsPackagedforDistribution))
    ;[1 1 1] Displaying the collider on game
    (Development|SetHiddeninGame (Variables|Default|GetDrillDetection_Head) false false)
    (Development|SetHiddeninGame (Variables|Default|GetDrillDetection_Body) false false))
  (Character|LaunchCharacter (* (Math|Vector|MakeVector _x 0.0 _y) (.drillimpulse (Variables|Data|GetCurrentUsedDrillInformation))) true true)
  (Variables|/Script/Engine.CharacterMovementComponent|SetbOrientRotationToMovement (Variables|Character|GetCharacterMovement) false)
  (if (> _x 0.0)
    (Transformation|SetActorRotation (Math|Rotator|MakeRotator 0.0 (* _returnvalue_8 -1.0) 0.0))
    (else
      (Transformation|SetActorRotation (Math|Rotator|MakeRotator 0.0 _returnvalue_8 0.0)))))

(fn AllowDrilling
  (Variables|Drill|SetcanPlayerDrill true))

(fn EndDrillingConfiguration
  (params (isEndByDrilling :type Boolean))
  (Development|PrintString "Entered to finish the drill" false)
  (Utilities|Time|ClearandInvalidateTimerbyHandle (Variables|Drill|GetEndDrillingTimer))
  (Variables|/Script/Engine.CharacterMovementComponent|SetGravityScale (Variables|Character|GetCharacterMovement) 1.0)
  (Variables|Drill|SetisDrilling false)
  (Variables|/Script/Engine.CharacterMovementComponent|SetbOrientRotationToMovement (Variables|Character|GetCharacterMovement) true)
  (Transformation|SetActorRotation (Math|Rotator|MakeRotator 0.0 0.0 (Variables|RotationInfo|GetPreviousRotationValue)))
  (Drill|ConsumeAllSpinsforDrill isEndByDrilling)
  (Variables|Movement|SetAimingDirection "(X=0.000000,Y=1.000000)")
  (Variables|Data|SetCurrentUsedDrillInformation "")
  (if (not (Class|KismetSystemLibrary|IsPackagedforDistribution))
    ;[1 1 1] Hiding the collider on game
    (Development|SetHiddeninGame (Variables|Default|GetDrillDetection_Head) true false)
    (Development|SetHiddeninGame (Variables|Default|GetDrillDetection_Body) true false)))

(fn RebounceCharacter
  (params (RebounceVector :type Vector%202D%20Structure :default "(X=0.000000,Y=0.000000)") (OverrideX_2D_Velocity :type Boolean) (OverrideY_2D_Velocity :type Boolean))
  (Character|LaunchCharacter (Math|Vector|MakeVector (.x RebounceVector) 0.0 (.y RebounceVector)) OverrideX_2D_Velocity OverrideY_2D_Velocity)
  (Development|PrintString (Utilities|String|Append "Rebounce performed With:   " "X:   " (Utilities|String|ToString(Float) (.x RebounceVector)) "   -   Y:   " (Utilities|String|ToString(Float) (.y RebounceVector))) false))

(fn DamageEnemy
  (params (EnemyToHarm :type BP%20Boss%20Object%20Reference))
  (bind _currentuseddrillinformation (Variables|Data|GetCurrentUsedDrillInformation))
  (if (not (Variables|/Game/Blueprints/Bosses/BP_Boss.BP_Boss_C|GetisInmune EnemyToHarm))
    (Game|Damage|ApplyDamage EnemyToHarm (.Value (Utilities|Map|Find (Variables|Data|GetDamageValuesBasedOnSpinLevel) (Variables|Drill|GetCurrentDrillLevel))) 0 0))
  (Default|ManualCameraShake (Variables|Movement|GetBP_Camera) "/Game/Blueprints/Camera/CameraShakeCurve_DefaultRotation.CameraShakeCurve_DefaultRotation" "/Game/Blueprints/Camera/CameraShakeCurve_DefaultLocation.CameraShakeCurve_DefaultLocation" 1.0 0.3)
  (Default|CallCallTimeDilation 0.0 0.2 true true false)
  (if (> (.x (Transformation|GetActorLocation)) (.x (Transformation|GetActorLocation EnemyToHarm)))
    (Movement|RebounceCharacter (Math|Vector2D|MakeVector2D (.x (.rebouncevectorwhenhittinganenemy _currentuseddrillinformation)) (.y (.rebouncevectorwhenhittinganenemy _currentuseddrillinformation))) true true)
    (Development|PrintString "Rebounce right" false)
    (else
      (Movement|RebounceCharacter (Math|Vector2D|MakeVector2D (* (.x (.rebouncevectorwhenhittinganenemy _currentuseddrillinformation)) -1.0) (.y (.rebouncevectorwhenhittinganenemy _currentuseddrillinformation))) true true)
      (Development|PrintString "Rebounce left" false))))

(fn UpdateHeadCollider
  (bind _drilldetection_head (Variables|Default|GetDrillDetection_Head))
  (bind _currentdrilllevel (Variables|Drill|GetCurrentDrillLevel))
  (bind _spininformationlevels (Variables|Data|GetSpinInformationLevels))
  (bind _output (Utilities|Array|Get(acopy) _spininformationlevels _currentdrilllevel))
  (Transformation|SetRelativeLocation _drilldetection_head (.location (.headcollidermodification _output)) false false)
  (Components|Capsule|SetCapsuleHalfHeight _drilldetection_head (.capsulehalfheight (.headcollidermodification _output)) true)
  (Components|Capsule|SetCapsuleRadius _drilldetection_head (.capsuleradius (.headcollidermodification _output)) true))

(fn CalculateRotationOftheSprite
  (bind _returnvalue (Transformation|GetActorRotation))
  (bind _returnvalue_2 (Math|Float|Absolute(Float) (.yaw _returnvalue)))
  (if (== (Variables|RotationInfo|GetPreviousRotationValue) _returnvalue_2)
    (Variables|RotationInfo|SetisRotating false)
    (else
      (Variables|RotationInfo|SetisRotating true)
      (if (> (Variables|RotationInfo|GetPreviousRotationValue) _returnvalue_2)
        (Variables|RotationInfo|SetisRotatingLeft false)
        (else
          (Variables|RotationInfo|SetisRotatingLeft true)))))
  (Variables|RotationInfo|SetPreviousRotationValue (.yaw _returnvalue)))

(fn HurtPlayerCharacter
  (Variables|Damaging|SetisInmune true)
  (CallFunction|SpawnVFXonCenter)
  (Movement|RebounceCharacter (Math|Vector2D|MakeVector2D (* (.x (Variables|Movement|GetAimingDirection)) -2e+02) 2e+02) true true)
  (Class|PaperZDAnimInstance|JumptoNode (Variables|/Script/PaperZD.PaperZDAnimationComponent|GetAnimInstance (Variables|Default|GetAnimationComponent)) "Hurted_Jump" "BasicStateMachine")
  (Class|PaperZDAnimInstance|JumptoNode (Variables|/Script/PaperZD.PaperZDAnimationComponent|GetAnimInstance (Variables|Default|GetPaperZDAnimation_Cone)) "HurtDrill_Jump" "Drill_StateMachine")
  (Default|ManualCameraShake (Variables|Movement|GetBP_Camera) "/Game/Blueprints/Camera/CameraShakeCurve_DefaultRotation.CameraShakeCurve_DefaultRotation" "/Game/Blueprints/Camera/CameraShakeCurve_DefaultLocation.CameraShakeCurve_DefaultLocation" 1.0 0.3)
  (Default|CallCallTimeDilation 0.0 0.2 true true true)
  (Drill|EndDrillingConfiguration false))

(fn EndDrilling
  (params (HasImpacted :type Boolean))
  (bind _animationcomponent (Variables|Default|GetAnimationComponent))
  (bind _animinstance (Variables|/Script/PaperZD.PaperZDAnimationComponent|GetAnimInstance _animationcomponent))
  (Utilities|FlowControl|DoOnce false :!label _label
    (:Completed
      (Drill|DrillCollisionsEnabling false)
      (Drill|EndDrillingConfiguration true)
      (if HasImpacted
        (Class|PaperZDAnimInstance|JumptoNode _animinstance "Impact_Jump" "BasicStateMachine")
        (else
          (Class|PaperZDAnimInstance|JumptoNode _animinstance "OnAir_Jump" "BasicStateMachine")))
      (bind _returnvalue (Utilities|Time|SetTimerbyEvent (EventDispatchers|CreateEvent :!event AllowDrilling) (Variables|Drill|GetDrillCooldown)))
      (Variables|Drill|SetDrillCooldownTimer _returnvalue)
      (goto _label Reset))))

(fn LaunchInmunityTimer
  (Utilities|Time|SetTimerbyEvent (EventDispatchers|CreateEvent :!event StopInmunity) (Variables|Damaging|GetInmuneTime))
  (CallFunction|StartInmunityFeel))

(fn StopInmunity
  (Variables|Damaging|SetisInmune false)
  (CallFunction|StopInmunityFeel))

(fn SpawnVFXonDrillTip
  (params (FlipbookToUse :type Paper%20Flipbook%20Object%20Reference) (YPosition :type Float%20%28double-precision%29))
  (Game|SpawnActorfromClass "/Game/Blueprints/Actors_VFX/BP_BasicImpactVFX.BP_BasicImpactVFX_C" (Math|Transform|MakeTransform (.location (Transformation|GetWorldTransform (Variables|Default|GetTipDrill_VFX))) "0, 0, 0" "1.000000,1.000000,1.000000") "AlwaysSpawn" "OverrideRootScale" 0 FlipbookToUse YPosition 0))

(fn SpawnVFXonCenter
  (Game|SpawnActorfromClass "/Game/Blueprints/Actors_VFX/BP_BasicImpactVFX.BP_BasicImpactVFX_C" (Math|Transform|MakeTransform (.location (Transformation|GetWorldTransform (Variables|Default|GetCenterCharacter))) "0, 0, 0" "1.000000,1.000000,1.000000") "AlwaysSpawn" "OverrideRootScale" 0 "/Game/Art/VFX/Animations/PC_Impact_VFX.PC_Impact_VFX" 1.4e+02 0))

(fn FingerAppearsandUpdatesPosition
  (bind _fingerreference (Variables|Finger|GetFingerReference))
  (Utilities|Time|ClearandInvalidateTimerbyHandle (Variables|Finger|GetFingerTimer))
  (Default|AppearFinger _fingerreference)
  (Default|UpdatePosition _fingerreference (Transformation|GetWorldLocation (Variables|Default|GetCenterCharacter)) (Variables|Movement|GetAimingDirection)))

(fn FingerHides
  (Default|HideFinger (Variables|Finger|GetFingerReference)))

(fn LaunchTimertoHideFinger
  (Default|UpdatePosition (Variables|Finger|GetFingerReference) (Transformation|GetWorldLocation (Variables|Default|GetCenterCharacter)) (Variables|Movement|GetAimingDirection))
  (Utilities|Time|SetTimerbyEvent (EventDispatchers|CreateEvent :!event FingerHides) (Variables|Finger|GetTimeToHideFinger)))
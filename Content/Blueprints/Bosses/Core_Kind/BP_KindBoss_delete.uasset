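; Sprite-based boss Blueprint that deals contact damage to BP_BossRushCharacter when its Box is overlapped.
; Taking damage triggers a two-color hit blink on registered sprites, using a material swap and chained timers before restoring the original look.
; Helpers toggle hitboxes and damage overlapping players through box, sphere or capsule checks, skipping immune or drilling characters.
; Another helper writes health to the Blackboard, but the health-changed event is empty.
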(event `self.Box.OnComponentBeginOverlap`
  (params (OverlappedComponent :type "PrimitiveComponent Object Reference") (OtherActor :type "Actor Object Reference") (OtherComp :type "PrimitiveComponent Object Reference") (OtherBodyIndex :type Integer) (bFromSweep :type Boolean) (SweepResult :type "HitResult Structure (by ref)"))
  (bind _asbp_boss_rush_character (cast `/Game/Blueprints/BP_BossRushCharacter` OtherActor))
  (`GameplayStatics.ApplyDamage` _asbp_boss_rush_character (`self.Base Damage`)))

(event `self.ReceiveBeginPlay`
  (`KismetSystemLibrary.Delay` 0.1)
  (set `self.OriginalSpriteColor` (`PaperFlipbookComponent.GetSpriteColor` (`self.Sprite`)))
  (add `self.OnTakeAnyDamage` (delegate `OnTakeAnyDamage_Event`))
  (`KismetArrayLibrary.Array_Add` (`self.BossSpritesToHitBlink`) (`self.Sprite`)))

(event `OnTakeAnyDamage_Event` :!signature `self.OnTakeAnyDamage`
  (params (DamagedActor :type "Actor Object Reference") (Damage :type "Float (single-precision)") (DamageType :type "DamageType Object Reference") (InstigatedBy :type "Controller Object Reference") (DamageCauser :type "Actor Object Reference"))
  (`self.HitBlinkStart` (`|GetArrayItem` (`self.HitBlinkColor`)) (`self.HitBlinkTime`)))

(event `self.BP_HealthComponent.OnHealthChanged`
  (params (NewHealth :type "Float (double-precision)")))

(fn `ActivateDeactivateCollider`
  (params (IsColliderActive :type Boolean) (BoxCollision :type "BoxComponent Object Reference"))
  (if IsColliderActive
    (`PrimitiveComponent.SetCollisionEnabled` BoxCollision "QueryOnly")
    (else
      (`PrimitiveComponent.SetCollisionEnabled` BoxCollision "NoCollision"))))

(fn `HitBlinkSecondColour`
  (for _array_element (`self.BossSpritesToHitBlink`)
    (`PaperFlipbookComponent.SetSpriteColor` _array_element (`|GetArrayItem` (`self.HitBlinkColor`) 1)))
  (`KismetSystemLibrary.K2_SetTimer` null "HitBlinkStop" (`self.HitBlinkTime`)))

(fn `HitBlinkStart`
  (params (Color :type "LinearColor Structure") (Time :type "Float (single-precision)"))
  (for _array_element (`self.BossSpritesToHitBlink`)
    (`PrimitiveComponent.SetMaterial` _array_element 0 (`self.HitBlinkMaterial`))
    (`PaperFlipbookComponent.SetSpriteColor` _array_element Color))
  (`KismetSystemLibrary.K2_SetTimer` null "HitBlinkSecondColour" Time))

(fn `HitBlinkStop`
  (for _array_element (`self.BossSpritesToHitBlink`)
    (`PrimitiveComponent.SetMaterial` _array_element 0 (`self.SpriteMaterial`))
    (`PaperFlipbookComponent.SetSpriteColor` _array_element (`self.OriginalSpriteColor`))))

(fn `SearchForCharacterInCollisionAndDamage_Box`
  (params (BoxCollision :type "BoxComponent Object Reference") (AttackDamage :type "Float (double-precision)"))
  (bind _overlappingactors (`PrimitiveComponent.GetOverlappingActors` BoxCollision "/Game/Blueprints/BP_BossRushCharacter.BP_BossRushCharacter_C"))
  (if (!= (`KismetArrayLibrary.Array_Length` _overlappingactors) 0)
    (bind _asbp_boss_rush_character (cast `/Game/Blueprints/BP_BossRushCharacter` (`|GetArrayItem` _overlappingactors)))
    (if (and (not (`/Game/Blueprints/BP_BossRushCharacter.isInmune` _asbp_boss_rush_character)) (not (`/Game/Blueprints/BP_BossRushCharacter.isDrilling` _asbp_boss_rush_character)))
      (`/Engine/EditorBlueprintResources/StandardMacros.DoOnce` false :!label _label
        (:`Completed`
          (`GameplayStatics.ApplyDamage` _asbp_boss_rush_character AttackDamage)
          (goto _label :!via `Reset`))))))

(fn `SearchForCharacterInCollisionAndDamage_Capsule`
  (params (Collision :type "CapsuleComponent Object Reference") (AttackDamage :type "Float (double-precision)"))
  (bind _overlappingactors (`PrimitiveComponent.GetOverlappingActors` Collision "/Game/Blueprints/BP_BossRushCharacter.BP_BossRushCharacter_C"))
  (if (!= (`KismetArrayLibrary.Array_Length` _overlappingactors) 0)
    (bind _asbp_boss_rush_character (cast `/Game/Blueprints/BP_BossRushCharacter` (`|GetArrayItem` _overlappingactors)))
    (if (and (not (`/Game/Blueprints/BP_BossRushCharacter.isInmune` _asbp_boss_rush_character)) (not (`/Game/Blueprints/BP_BossRushCharacter.isDrilling` _asbp_boss_rush_character)))
      (`/Engine/EditorBlueprintResources/StandardMacros.DoOnce` false :!label _label
        (:`Completed`
          (`GameplayStatics.ApplyDamage` _asbp_boss_rush_character AttackDamage)
          (goto _label :!via `Reset`))))))

(fn `SearchForCharacterInCollisionAndDamage_Sphere`
  (params (Collision :type "SphereComponent Object Reference") (AttackDamage :type "Float (double-precision)"))
  (bind _overlappingactors (`PrimitiveComponent.GetOverlappingActors` Collision "/Game/Blueprints/BP_BossRushCharacter.BP_BossRushCharacter_C"))
  (if (!= (`KismetArrayLibrary.Array_Length` _overlappingactors) 0)
    (bind _asbp_boss_rush_character (cast `/Game/Blueprints/BP_BossRushCharacter` (`|GetArrayItem` _overlappingactors)))
    (if (and (not (`/Game/Blueprints/BP_BossRushCharacter.isInmune` _asbp_boss_rush_character)) (not (`/Game/Blueprints/BP_BossRushCharacter.isDrilling` _asbp_boss_rush_character)))
      (`/Engine/EditorBlueprintResources/StandardMacros.DoOnce` false :!label _label
        (:`Completed`
          (`GameplayStatics.ApplyDamage` _asbp_boss_rush_character AttackDamage)
          (goto _label :!via `Reset`))))))

(fn `UpdateBlackboardHealthValue`
  (params (NewHealth :type "Float (double-precision)"))
  (locals (RemainingHealth_KeyBlackboard :type Name :default "RemainingHealth"))
  (`BlackboardComponent.SetValueAsFloat` (`AIBlueprintHelperLibrary.GetBlackboard` null) (`local.RemainingHealth_KeyBlackboard`) NewHealth))

(fn `UserConstructionScript`)
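; Mole boss for a boss-rush fight that pops up at appear points to peek, flip or throw trash.
; Its AI controller runs the behaviour tree and health changes update the blackboard.
; Attacks activate a random or player-nearest point, then teleport the boss and jump animation state-machine nodes.
; Flip movement uses timelines lerping X and Z, while trash throwing exits after counting destroyed pieces.
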(event `self.ReceiveBeginPlay`
  (add `self.TrashDestroyed` (`|CreateDelegate` :!event `TrashDestroyedCheck`))
  (bind _returnvalue (`GameplayStatics.GetActorOfClass` "/Game/Blueprints/BP_BossRushCharacter.BP_BossRushCharacter_C"))
  (`/Engine/EditorBlueprintResources/StandardMacros.IsValid` _returnvalue
    (:`Is Valid`
      (set `self.PlayerCharacter` _returnvalue))
    (:`Is Not Valid`
      _))
  (`parent.ReceiveBeginPlay`)
  (`KismetArrayLibrary.Array_Add` (`self.BossSpritesToHitBlink`) (`self.MoleHands_Flipbook`)))

(event `self.BP_HealthComponent.OnHealthChanged`
  (params (NewHealth :type "Float (double-precision)"))
  (bind _returnvalue (`self.K2_GetActorLocation`))
  (`self.UpdateBlackboardHealthValue` NewHealth)
  (`/Game/Audio/BPFL_Audio.PlayRandom3DSound` (`|MakeArray` "/Game/Audio/Assets/SFX/Characters/Molenius/Mol_Damage_Hit-001.Mol_Damage_Hit-001" "/Game/Audio/Assets/SFX/Characters/Molenius/Mol_Damage_Hit-002.Mol_Damage_Hit-002" "/Game/Audio/Assets/SFX/Characters/Molenius/Mol_Damage_Hit-003.Mol_Damage_Hit-003" :!type "SoundBase Object Reference") "/Game/Audio/MainAttenuation.MainAttenuation" _returnvalue)
  (`/Game/Audio/BPFL_Audio.PlayRandom3DSound` (`|MakeArray` "/Game/Audio/Assets/SFX/Characters/Molenius/Mol_Damage_Vocal-001.Mol_Damage_Vocal-001" "/Game/Audio/Assets/SFX/Characters/Molenius/Mol_Damage_Vocal-002.Mol_Damage_Vocal-002" :!type "SoundBase Object Reference") "/Game/Audio/MainAttenuation.MainAttenuation" _returnvalue))

(event `self.BP_HealthComponent.OnDeath`
  (`self.ManageBossDeath`))

(event `PerformFlipAttack_Event`
  (bind (_returnvalue_x _returnvalue_y) (`KismetMathLibrary.BreakVector` (`self.K2_GetActorLocation`)))
  (bind _selectedpositiontoappear (`self.SelectedPositionToAppear`))
  (bind _returnvalue (`SceneComponent.K2_GetComponentLocation` (`/Game/Blueprints/Bosses/MoleBoss/BP_AppearancePoint.StartingPoint` _selectedpositiontoappear)))
  (bind (_returnvalue_x_2 _returnvalue_y_2 _returnvalue_z) (`KismetMathLibrary.BreakVector` (`SceneComponent.K2_GetComponentLocation` (`/Game/Blueprints/Bosses/MoleBoss/BP_AppearancePoint.FlipPosition` _selectedpositiontoappear))))
  (`PaperZDAnimInstance.JumpToNode` (`PaperZDAnimationComponent.AnimInstance` (`self.AnimationComponent`)) "StartFlip_Jump" "MoleBoss_StateMachine")
  (`self.K2_SetActorTransform` (`KismetMathLibrary.MakeTransform` _returnvalue (`self.K2_GetActorRotation` _selectedpositiontoappear)) false true)
  (bind (_direction _completition) (`Timeline|GoingToPointFlipAttack` :!via `PlayFromStart`)
    (:`Update`
      (`self.K2_SetActorLocation` (`KismetMathLibrary.MakeVector` (`KismetMathLibrary.Lerp` (.x _returnvalue) _returnvalue_x_2 _completition) _returnvalue_y (`KismetMathLibrary.Lerp` (.z _returnvalue) _returnvalue_z _completition))))
    (:`Finished`
      (`PaperZDAnimInstance.JumpToNode` (`PaperZDAnimationComponent.AnimInstance` (`self.AnimationComponent`)) "PerformFlip_Jump" "MoleBoss_StateMachine"))))

(event `ReturnToStartPoint_Event`
  (bind (_returnvalue_x _returnvalue_y) (`KismetMathLibrary.BreakVector` (`self.K2_GetActorLocation`)))
  (bind _selectedpositiontoappear (`self.SelectedPositionToAppear`))
  (bind (_returnvalue_x_2 _returnvalue_y_2 _returnvalue_z) (`KismetMathLibrary.BreakVector` (`SceneComponent.K2_GetComponentLocation` (`/Game/Blueprints/Bosses/MoleBoss/BP_AppearancePoint.StuckInPlace` _selectedpositiontoappear))))
  (bind (_returnvalue_x_3 _returnvalue_y_3 _returnvalue_z_2) (`KismetMathLibrary.BreakVector` (`SceneComponent.K2_GetComponentLocation` (`/Game/Blueprints/Bosses/MoleBoss/BP_AppearancePoint.FlipPosition` _selectedpositiontoappear))))
  (bind (_direction _completition) (`Timeline|Timeline` :!via `PlayFromStart`)
    (:`Update`
      (`self.K2_SetActorLocation` (`KismetMathLibrary.MakeVector` (`KismetMathLibrary.Lerp` _returnvalue_x_3 _returnvalue_x_2 _completition) _returnvalue_y (`KismetMathLibrary.Lerp` _returnvalue_z_2 _returnvalue_z _completition))))
    (:`Finished`
      (`PaperZDAnimInstance.JumpToNode` (`PaperZDAnimationComponent.AnimInstance` (`self.AnimationComponent`)) "ExitingFlip_Jump" "MoleBoss_StateMachine"))))

(fn `HideMoleBoss`
  (`/Game/Blueprints/Bosses/MoleBoss/BP_AppearancePoint.Appear Point Deactivate` (`self.SelectedPositionToAppear`))
  (`self.K2_SetActorLocation` (500.0 500.0 500.0) false true)
  (`self.K2_SetActorRotation` (struct)))

(fn `ManageBossDeath`
  (`PrimitiveComponent.SetCollisionObjectType` (`self.CapsuleComponent`) "ECC_WorldStatic")
  (`parent.ManageBossDeath`))

(fn `PerformDeath`
  (bind _selectedpositiontoappear (`self.SelectedPositionToAppear`))
  (`self.K2_SetActorTransform` (`KismetMathLibrary.MakeTransform` (`self.K2_GetActorLocation` _selectedpositiontoappear) (`self.K2_GetActorRotation` _selectedpositiontoappear)) false true)
  (`PaperZDAnimInstance.JumpToNode` (`PaperZDAnimationComponent.AnimInstance` (`self.AnimationComponent`)) "Death_Jump" "MoleBoss_StateMachine"))

(fn `PerformPeekAttack`
  (bind _selectedpositiontoappear (`self.SelectedPositionToAppear`))
  (`self.K2_SetActorTransform` (`KismetMathLibrary.MakeTransform` (`self.K2_GetActorLocation` _selectedpositiontoappear) (`self.K2_GetActorRotation` _selectedpositiontoappear)) false true)
  (`PaperZDAnimInstance.JumpToNode` (`PaperZDAnimationComponent.AnimInstance` (`self.AnimationComponent`)) "Peek_Jump" "MoleBoss_StateMachine"))

(fn `PerformThrowTrashAttack`
  (params (TrashToThrowPerSide :type Integer))
  (bind _selectedpositiontoappear (`self.SelectedPositionToAppear`))
  (set `self.Trash to Throw Per Side` TrashToThrowPerSide)
  (`self.K2_SetActorTransform` (`KismetMathLibrary.MakeTransform` (`self.K2_GetActorLocation` _selectedpositiontoappear) (`self.K2_GetActorRotation` _selectedpositiontoappear)) false true)
  (`PaperZDAnimInstance.JumpToNode` (`PaperZDAnimationComponent.AnimInstance` (`self.AnimationComponent`)) "ThrowTrash_Jump" "MoleBoss_StateMachine"))

(fn `SelectNearToPlayerAppearPosition`
  (locals (currentSelectedPosition :type "/Game/Blueprints/Bosses/MoleBoss/BP_AppearancePoint Object Reference") (currentMinimumDistance :type "Float (double-precision)" :default 1000000000.0))
  (for _array_element (`self.AppearPositions`)
    (bind _returnvalue (`KismetMathLibrary.Vector_Distance` (`self.K2_GetActorLocation` (`self.PlayerCharacter`)) (`self.K2_GetActorLocation` _array_element)))
    (if (<= _returnvalue (`local.currentMinimumDistance`))
      (set `local.currentSelectedPosition` _array_element)
      (set `local.currentMinimumDistance` _returnvalue)))
  (set `self.SelectedPositionToAppear` (`local.currentSelectedPosition`)))

(fn `SelectRandomAppearPosition`
  (bind _appearpositions (`self.AppearPositions`))
  (set `self.SelectedPositionToAppear` (`|GetArrayItem` _appearpositions (`KismetMathLibrary.RandomIntegerInRange` 0 (- (`KismetArrayLibrary.Array_Length` _appearpositions) 1)))))

(fn `StartDeath`
  (`/Game/Blueprints/Bosses/MoleBoss/BP_AppearancePoint.AppearPointActivate` (`self.SelectedPositionToAppear`)))

(fn `StartFightConfiguration`
  (bind _asbp_ai_controller_mole_boss (cast `/Game/Blueprints/Bosses/MoleBoss/BP_AiController_MoleBoss` (`self.GetController`)))
  (`/Game/Blueprints/Bosses/MoleBoss/BP_AiController_MoleBoss.RunMoleniusBehaviourTree` _asbp_ai_controller_mole_boss)
  (`self.UpdateBlackboardHealthValue` (`/Game/Blueprints/Components/BP_HealthComponent.MaxHealth` (`self.BP_HealthComponent`))))

(fn `StartPerformingFlipAttack`
  (params (IsRandomPosition :type Boolean))
  (if IsRandomPosition
    (`self.SelectRandomAppearPosition`)
    (else
      (`self.SelectNearToPlayerAppearPosition`)))
  (`/Game/Blueprints/Bosses/MoleBoss/BP_AppearancePoint.AppearPointActivate` (`self.SelectedPositionToAppear`)))

(fn `StartPerformingPeekAttack`
  (params (isRAndomPosition :type Boolean))
  (if isRAndomPosition
    (`self.SelectRandomAppearPosition`)
    (else
      (`self.SelectNearToPlayerAppearPosition`)))
  (`/Game/Blueprints/Bosses/MoleBoss/BP_AppearancePoint.AppearPointActivate` (`self.SelectedPositionToAppear`)))

(fn `StartPerformingThrowTrashAttack`
  (params (IsRandomPosition :type Boolean))
  (if IsRandomPosition
    (`self.SelectRandomAppearPosition`)
    (else
      (`self.SelectNearToPlayerAppearPosition`)))
  (`/Game/Blueprints/Bosses/MoleBoss/BP_AppearancePoint.AppearPointActivate` (`self.SelectedPositionToAppear`)))

(fn `TrashDestroyedCheck`
  (bind _result (`/Engine/EditorBlueprintResources/StandardMacros.IncrementInt` (`self.CurrentDestroyedTrash`))
    (:`  `
      (if (>= _result (* (`self.Trash to Throw Per Side`) 2))
        (set `self.CurrentDestroyedTrash` 0)
        (`PaperZDAnimInstance.JumpToNode` (`PaperZDAnimationComponent.AnimInstance` (`self.AnimationComponent`)) "Throwtrash_Exit_Jump" "MoleBoss_StateMachine")))))

(fn `UserConstructionScript`
  (`SceneComponent.SetVisibility` (`self.MoleHands_Flipbook`) false false)
  (`parent.UserConstructionScript`))
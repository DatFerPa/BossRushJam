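; BP_MovableMap_delete is a map actor that lowers itself from an initial location to a final location after BeginPlay.
; MoveMap loops on a short Delay, stepping the actor down the Z axis without sweep until its position exactly matches the target, with zero tolerance.
; A separate function calls EndDrilling on a supplied boss rush character.
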(event `self.ReceiveBeginPlay`
  (`self.MoveMap`))

(event `MoveMap`
  (set `self.RealLocation` (`self.InitialLocation`))
  (if (`self.IsFinalLocation`) :!label _label
    _
    (elif (== (`self.RealLocation`) (`self.FinalLocation`))
      (set `self.IsFinalLocation` true)
      (goto _label)
      (else
        (`KismetSystemLibrary.Delay` 0.01)
        (bind _output_get (set `self.RealLocation` (- (`self.RealLocation`) (0.0 0.0 1.0))))
        (`self.K2_SetActorLocation` _output_get)
        (goto _label)))))

(fn `Call PlayerActionWhenDrilling`
  (params (BPBossRushCharacter :type "/Game/Blueprints/BP_BossRushCharacter Object Reference"))
  (`/Game/Blueprints/BP_BossRushCharacter.EndDrilling` BPBossRushCharacter true))

(fn `UserConstructionScript`)
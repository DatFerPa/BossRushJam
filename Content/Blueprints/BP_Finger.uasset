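; BP_Finger is a 2D flipbook finger actor that points along an aiming direction from a supplied character position.
; UpdatePosition moves it to that position and derives pitch from the angle between the aim vector, mirrored to positive X, and the X axis.
; Pitch is negated for downward aim, and a 180-degree yaw flips the finger for leftward aim.
; HideFinger and AppearFinger toggle the flipbook's visibility; the actor has no active event logic.
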(event `self.ReceiveBeginPlay`)

(fn `AppearFinger`
  (`SceneComponent.SetVisibility` (`self.Finger_FlipBook`) true false))

(fn `HideFinger`
  (`SceneComponent.SetVisibility` (`self.Finger_FlipBook`) false false))

(fn `UpdatePosition`
  (params (CharacterTransform :type "Vector Structure") (AimingDirection :type "Vector2D Structure"))
  (locals (Rotation_Y :type "Float (double-precision)") (Rotation_Z :type "Float (double-precision)"))
  (bind _returnvalue (`KismetMathLibrary.MakeVector2D` 1.0))
  (bind (_x _y) (`KismetMathLibrary.BreakVector2D` AimingDirection))
  (bind (_x_2 _y_2) (`KismetMathLibrary.BreakVector2D` AimingDirection))
  (bind _returnvalue_2 (`KismetMathLibrary.MakeVector2D` (`KismetMathLibrary.Abs` _x) _y))
  (`self.K2_SetActorLocation` CharacterTransform)
  (set `local.Rotation_Y` (`KismetMathLibrary.DegAcos` (/ (`KismetMathLibrary.DotProduct2D` _returnvalue _returnvalue_2) (* (`KismetMathLibrary.VSize2D` _returnvalue) (`KismetMathLibrary.VSize2D` _returnvalue_2)))))
  (if (not (>= _x_2 0.0))
    (set `local.Rotation_Z` -180.0))
  (if (not (>= _y_2 0.0))
    (set `local.Rotation_Y` (* (`local.Rotation_Y`) -1.0)))
  (`self.K2_SetActorRotation` (`KismetMathLibrary.MakeRotator` 0.0 (`local.Rotation_Y`) (`local.Rotation_Z`))))

(fn `UserConstructionScript`)
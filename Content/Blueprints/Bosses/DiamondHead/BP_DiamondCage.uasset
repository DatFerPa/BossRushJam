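; BP_DiamondCage is a DiamondHead boss attack: a telegraphed cage of three walls that damages the player caught inside.
; On BeginPlay it creates dynamic debug materials for the walls and runs a timeline that animates their opacity as anticipation.
; When the timeline finishes, the walls turn red and the damage collision applies cage damage if it overlaps the player.
; Either way, the actor destroys itself after a short delay.
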(event `self.ReceiveBeginPlay`
  (bind _returnvalue (`PrimitiveComponent.CreateDynamicMaterialInstance` (`self.CubeWall1`) 0 "/Game/Blueprints/Bosses/DiamondHead/DebugMaterial.DebugMaterial" "None"))
  (`KismetArrayLibrary.Array_AddUnique` (`self.WallsDynamicMaterials`) _returnvalue)
  (bind _returnvalue_2 (`PrimitiveComponent.CreateDynamicMaterialInstance` (`self.CubeWall2`) 0 "/Game/Blueprints/Bosses/DiamondHead/DebugMaterial.DebugMaterial" "None"))
  (`KismetArrayLibrary.Array_AddUnique` (`self.WallsDynamicMaterials`) _returnvalue_2)
  (bind _returnvalue_3 (`PrimitiveComponent.CreateDynamicMaterialInstance` (`self.CubeWall3`) 0 "/Game/Blueprints/Bosses/DiamondHead/DebugMaterial.DebugMaterial" "None"))
  (`KismetArrayLibrary.Array_AddUnique` (`self.WallsDynamicMaterials`) _returnvalue_3)
  (bind (_direction _opacity) (`Timeline|AttackAnticipation` :!via `PlayFromStart`)
    (:`Update`
      (`MeshComponent.SetScalarParameterValueOnMaterials` (`self.CubeWall3`) "Opacity" _opacity)
      (`MeshComponent.SetScalarParameterValueOnMaterials` (`self.CubeWall2`) "Opacity" _opacity)
      (`MeshComponent.SetScalarParameterValueOnMaterials` (`self.CubeWall1`) "Opacity" _opacity))
    (:`Finished`
      (`self.PerformAttack`))))

(event `DelayedDestruction`
  (`KismetSystemLibrary.Delay` 0.5)
  (`self.K2_DestroyActor`))

(fn `PerformAttack`
  (for _array_element (`self.WallsDynamicMaterials`)
    (`MaterialInstanceDynamic.SetVectorParameterValue` _array_element "ColorParameter" (struct :`R` 1.0 :`A` 1.0)))
  (if (== (`|GetArrayItem` (`PrimitiveComponent.GetOverlappingActors` (`self.DamageCollision`) "/Game/Blueprints/BP_BossRushCharacter.BP_BossRushCharacter_C")) (`self.PlayerCharacter`))
    (`GameplayStatics.ApplyDamage` (`self.PlayerCharacter`) (`self.CageDamage`))
    (`self.DelayedDestruction`)
    (else
      (`self.DelayedDestruction`))))

(fn `UserConstructionScript`)
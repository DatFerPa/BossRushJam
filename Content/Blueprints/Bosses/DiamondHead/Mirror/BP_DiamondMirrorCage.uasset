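; Mirror cage hazard for the Diamond Head boss that appears, attacks after a delay and damages the player.
; PaperZD animation jumps play the appear state on BeginPlay and the attack state once PerformDelayedAttack's delay ends.
; DamageCollision overlaps apply cage damage unless the player is drilling or immune.
; Small functions toggle that hurtbox and destroy the actor, with no callers in this Blueprint.
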(event `self.ReceiveBeginPlay`
  (bind _output_get (set `self.ABP` (`PaperZDAnimationComponent.AnimInstance` (`self.PaperZDAnimation`))))
  (`PaperZDAnimInstance.JumpToNode` _output_get "JumpMirrorAppear" "None"))

(event `PerformDelayedAttack`
  (`KismetSystemLibrary.Delay` (`self.AttackDelay`))
  (`PaperZDAnimInstance.JumpToNode` (`self.ABP`) "JumpMirrorAttack" "None"))

(event `self.DamageCollision.OnComponentBeginOverlap`
  (params (OverlappedComponent :type "PrimitiveComponent Object Reference") (OtherActor :type "Actor Object Reference") (OtherComp :type "PrimitiveComponent Object Reference") (OtherBodyIndex :type Integer) (bFromSweep :type Boolean) (SweepResult :type "HitResult Structure (by ref)"))
  (bind _playercharacter (`self.PlayerCharacter`))
  (if (and (== OtherActor _playercharacter) (not (`/Game/Blueprints/BP_BossRushCharacter.isDrilling` _playercharacter)) (not (`/Game/Blueprints/BP_BossRushCharacter.isInmune` _playercharacter)))
    (`GameplayStatics.ApplyDamage` (`self.PlayerCharacter`) (`self.CageDamage`))))

(fn `ActivateHurtbox`
  (`PrimitiveComponent.SetCollisionEnabled` (`self.DamageCollision`) "QueryAndPhysics"))

(fn `DisableHurtbox`
  (`PrimitiveComponent.SetCollisionEnabled` (`self.DamageCollision`) "NoCollision"))

(fn `SelfDestroy`
  (`self.K2_DestroyActor`))

(fn `UserConstructionScript`)
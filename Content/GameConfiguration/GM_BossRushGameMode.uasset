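; Game mode for the boss rush that sets the view camera, creates the HUD, and caches player, boss, map and background.
; It provides timed hit-stop style slowdowns through CustomTimeDilation, applied selectively to player, boss or tracked projectiles rather than global dilation.
; On player death it freezes all three, hides the map, flashes sprites and background red and white, then resumes only the player for the death animation.
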(event `self.ReceiveBeginPlay`
  (`|ExecutionSequence`
    (:`then_0`
      ;[1 1 1] Configuring the camera
      (bind _returnvalue (`GameplayStatics.GetActorOfClass` "/Game/Blueprints/Camera/BP_Camera.BP_Camera_C"))
      (`/Engine/EditorBlueprintResources/StandardMacros.IsValid` _returnvalue
        (:`Is Valid`
          (bind _output_get (set `self.BP_Camera` _returnvalue))
          (`PlayerController.SetViewTargetWithBlend` (`GameplayStatics.GetPlayerController` 0) _output_get 0.0 "VTBlend_Linear" 0.0 false))
        (:`Is Not Valid`
          _))
      ;[1 1 1] Binding to the Time Dilation Event
      (bind _returnvalue_2 (`GameplayStatics.GetActorOfClass` "/Game/Blueprints/BP_BossRushCharacter.BP_BossRushCharacter_C"))
      (`/Engine/EditorBlueprintResources/StandardMacros.IsValid` _returnvalue_2
        (:`Is Valid`
          (bind _output_get_2 (set `self.BP_PlayerCharacter` _returnvalue_2))
          (add `/Game/Blueprints/BP_BossRushCharacter.CallTimeDilation` _output_get_2 (`|CreateDelegate` :!event `ChangeDilation`)))
        (:`Is Not Valid`
          _))
      ;[1 1 1] Linking Boss
      (bind _returnvalue_3 (`GameplayStatics.GetActorOfClass` "/Game/Blueprints/Bosses/BP_Boss.BP_Boss_C"))
      (`/Engine/EditorBlueprintResources/StandardMacros.IsValid` _returnvalue_3
        (:`Is Valid`
          (set `self.BP_Boss` _returnvalue_3))))
    (:`then_1`
      ;[1 1 1] Creating the HUD
      (bind _returnvalue_4 (`|CreateWidget` "/Game/UI/WBP_HUD.WBP_HUD_C"))
      (bind _output_get_3 (set `self.WBP_HUD` _returnvalue_4))
      (`UserWidget.AddToViewport` _output_get_3 0))
    (:`then_2`
      (add `/Game/Blueprints/BP_BossRushCharacter.PlayerDeath` (`self.BP_PlayerCharacter`) (delegate `ManageDeath`))
      (bind _returnvalue_5 (`GameplayStatics.GetActorOfClass` "/Game/Blueprints/Map/BP_BasicMap.BP_BasicMap_C"))
      (set `self.Map` _returnvalue_5)
      (bind _returnvalue_6 (`GameplayStatics.GetActorOfClass` "/Game/Art/Environment/DeathBackGround/BP_Background.BP_Background_C"))
      (set `self.Background` _returnvalue_6))))

(event `ManageDeath`
  (bind _bp_playercharacter (`self.BP_PlayerCharacter`))
  (bind _bp_playercharacter_2 (`self.BP_PlayerCharacter`))
  (bind _bp_playercharacter_3 (`self.BP_PlayerCharacter`))
  (bind _bp_playercharacter_4 (`self.BP_PlayerCharacter`))
  (bind _sprite (`PaperCharacter.Sprite` _bp_playercharacter_2))
  (bind _conedrill_flipbook (`/Game/Blueprints/BP_BossRushCharacter.ConeDrill_Flipbook` _bp_playercharacter_2))
  (bind _sprite_2 (`PaperCharacter.Sprite` _bp_playercharacter_4))
  (bind _conedrill_flipbook_2 (`/Game/Blueprints/BP_BossRushCharacter.ConeDrill_Flipbook` _bp_playercharacter_4))
  (`self.ChangeOtherActorsDilation` 0.0)
  (`self.Change Player Character Dilation` 0.0)
  (`self.ChangeBossDilation` 0.0)
  (`PrimitiveComponent.SetMaterial` _sprite 0 "/Game/Art/materials/MT_HitMaterial.MT_HitMaterial")
  (`PrimitiveComponent.SetMaterial` _conedrill_flipbook 0 "/Game/Art/materials/MT_HitMaterial.MT_HitMaterial")
  (`PaperFlipbookComponent.SetSpriteColor` _conedrill_flipbook (struct :`R` 1.0 :`G` 1.0 :`B` 1.0 :`A` 1.0))
  (`PaperFlipbookComponent.SetSpriteColor` _sprite (struct :`R` 1.0 :`G` 1.0 :`B` 1.0 :`A` 1.0))
  (`PaperFlipbookComponent.SetSpriteColor` (`/Game/Art/Environment/DeathBackGround/BP_Background.PaperFlipbook` (`self.Background`)) (struct :`R` 1.0 :`A` 1.0))
  (`SceneComponent.SetVisibility` (`/Game/Blueprints/Map/BP_BasicMap.DefaultSceneRoot` (`self.Map`)) false true)
  (`/Game/Blueprints/Bosses/BP_Boss.ApplyMaterialChange` (`self.BP_Boss`) (struct :`R` 1.0 :`G` 1.0 :`B` 1.0 :`A` 1.0))
  (`KismetSystemLibrary.Delay` 0.5)
  (`PaperFlipbookComponent.SetSpriteColor` (`PaperCharacter.Sprite` _bp_playercharacter) (struct :`R` 1.0 :`A` 1.0))
  (`PaperFlipbookComponent.SetSpriteColor` (`/Game/Blueprints/BP_BossRushCharacter.ConeDrill_Flipbook` _bp_playercharacter) (struct :`R` 1.0 :`A` 1.0))
  (`/Game/Blueprints/Bosses/BP_Boss.ApplyMaterialChange` (`self.BP_Boss`) (struct :`R` 1.0 :`A` 1.0))
  (`PaperFlipbookComponent.SetSpriteColor` (`/Game/Art/Environment/DeathBackGround/BP_Background.PaperFlipbook` (`self.Background`)) (struct :`R` 1.0 :`G` 1.0 :`B` 1.0 :`A` 1.0))
  (`KismetSystemLibrary.Delay` 0.5)
  (`PrimitiveComponent.SetMaterial` _sprite_2 0 "/Game/Art/materials/MT_SpriteMaterial.MT_SpriteMaterial")
  (`PrimitiveComponent.SetMaterial` _conedrill_flipbook_2 0 "/Game/Art/materials/MT_SpriteMaterial.MT_SpriteMaterial")
  (`PaperFlipbookComponent.SetSpriteColor` _conedrill_flipbook_2 (struct :`R` 1.0 :`G` 1.0 :`B` 1.0 :`A` 1.0))
  (`PaperFlipbookComponent.SetSpriteColor` _sprite_2 (struct :`R` 1.0 :`G` 1.0 :`B` 1.0 :`A` 1.0))
  (`PaperFlipbookComponent.SetSpriteColor` (`/Game/Art/Environment/DeathBackGround/BP_Background.PaperFlipbook` (`self.Background`)) (struct :`R` 0.026042 :`G` 0.026042 :`B` 0.026042 :`A` 1.0))
  (`/Game/Blueprints/Bosses/BP_Boss.HitBlinkStop` (`self.BP_Boss`))
  (`self.Change Player Character Dilation` 1.0)
  (`SceneComponent.SetVisibility` (`/Game/Blueprints/BP_BossRushCharacter.ConeDrill_Flipbook` _bp_playercharacter_3) false false)
  (`PaperZDAnimInstance.JumpToNode` (`PaperZDAnimationComponent.AnimInstance` (`PaperZDCharacter.AnimationComponent` _bp_playercharacter_3)) "PlayerDeath_Jump" "BasicStateMachine"))

(fn `Change Player Character Dilation`
  (params (TimeDilation :type "Float (double-precision)"))
  (set `Actor.CustomTimeDilation` TimeDilation (`self.BP_PlayerCharacter`)))

(fn `ChangeBossDilation`
  (params (TimeDilation :type "Float (double-precision)"))
  (set `Actor.CustomTimeDilation` TimeDilation (`self.BP_Boss`)))

(fn `ChangeDilation`
  (params (TimeDilation :type "Float (double-precision)") (AmountOfTimeDilatingTime :type "Float (double-precision)") (AffectPlayer :type Boolean) (AffectBoss :type Boolean) (AffectOtherActors :type Boolean))
  (`KismetSystemLibrary.K2_ClearAndInvalidateTimerHandle` (`self.TimeDilation_Timer`))
  (if AffectPlayer
    (`self.Change Player Character Dilation` TimeDilation))
  (if AffectBoss
    (`self.ChangeBossDilation` TimeDilation))
  (if AffectOtherActors
    (`self.ChangeOtherActorsDilation` TimeDilation))
  (bind _returnvalue (`KismetSystemLibrary.K2_SetTimerDelegate` (`|CreateDelegate` :!event `EndGlobalDilation`) AmountOfTimeDilatingTime))
  (set `self.TimeDilation_Timer` _returnvalue))

(fn `ChangeOtherActorsDilation`
  (params (Dilation :type "Float (double-precision)"))
  (for _array_element (`self.Projectiles`)
    (set `Actor.CustomTimeDilation` Dilation _array_element)))

(fn `EndGlobalDilation`
  (`self.ChangeBossDilation` 1.0)
  (`self.Change Player Character Dilation` 1.0)
  (`self.ChangeOtherActorsDilation` 1.0))

(fn `UserConstructionScript`)
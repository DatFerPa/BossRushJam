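; Diamond Head boss with a close-range "Erizo" attack and waypoint repositioning.
; ErizoCollider overlaps set the PlayerInErizoRange blackboard flag as the player enters or leaves.
; Anticipation starts a timer, and ErizoAttack damages the first overlapping player unless immune or drilling.
; MoveToAnotherPoint jumps the boss to a random waypoint in the opposite pair, based on CurrentWaypoint.
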(event `self.ErizoCollider.OnComponentBeginOverlap`
  (params (OverlappedComponent :type "PrimitiveComponent Object Reference") (OtherActor :type "Actor Object Reference") (OtherComp :type "PrimitiveComponent Object Reference") (OtherBodyIndex :type Integer) (bFromSweep :type Boolean) (SweepResult :type "HitResult Structure (by ref)"))
  ;[1 1 1] Player in Erizo Range
  (cast `/Game/Blueprints/BP_BossRushCharacter` OtherActor)
  (`BlackboardComponent.SetValueAsBool` (`AIBlueprintHelperLibrary.GetBlackboard` null) "PlayerInErizoRange" true))

(event `self.ErizoCollider.OnComponentEndOverlap`
  (params (OverlappedComponent :type "PrimitiveComponent Object Reference") (OtherActor :type "Actor Object Reference") (OtherComp :type "PrimitiveComponent Object Reference") (OtherBodyIndex :type Integer))
  ;[1 1 1] Player in Erizo Range
  (cast `/Game/Blueprints/BP_BossRushCharacter` OtherActor)
  (`BlackboardComponent.SetValueAsBool` (`AIBlueprintHelperLibrary.GetBlackboard` null) "PlayerInErizoRange" false))

(fn `ErizoAttack`
  (bind _output (`|GetArrayItem` (`PrimitiveComponent.GetOverlappingActors` (`self.ErizoCollider`) "/Game/Blueprints/BP_BossRushCharacter.BP_BossRushCharacter_C")))
  (`/Engine/EditorBlueprintResources/StandardMacros.IsValid` _output
    (:`Is Valid`
      (bind _asbp_boss_rush_character (cast `/Game/Blueprints/BP_BossRushCharacter` _output))
      (if (and (not (`/Game/Blueprints/BP_BossRushCharacter.isInmune` _asbp_boss_rush_character)) (not (`/Game/Blueprints/BP_BossRushCharacter.isDrilling` _asbp_boss_rush_character)))
        (`GameplayStatics.ApplyDamage` _asbp_boss_rush_character (`self.ErizoDamage`))))))

(fn `MoveToAnotherPoint`
  (if (< (`self.CurrentWaypoint`) 2)
    (`self.K2_SetActorLocation` (`self.K2_GetActorLocation` (`|GetArrayItem` (`self.Waypoints`) (`KismetMathLibrary.RandomIntegerInRange` 2 3))))
    (else
      (`self.K2_SetActorLocation` (`self.K2_GetActorLocation` (`|GetArrayItem` (`self.Waypoints`) (`KismetMathLibrary.RandomIntegerInRange` 0 1)))))))

(fn `StartErizoAnticipation`
  (`KismetSystemLibrary.K2_SetTimerDelegate` (`|CreateDelegate` :!event `ErizoAttack`) (`self.ErizoAnticipationTime`)))

(fn `UserConstructionScript`
  (`parent.UserConstructionScript`))
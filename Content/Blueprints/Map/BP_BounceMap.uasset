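; BP_BounceMap is a map element that bounces a drilling player character off it.
; It overrides the parent's drilling response: at or above the required drill level, it plays an impact VFX on the drill tip and drills the character in a reflected direction.
; The reflection negates one component of the aiming direction, chosen by the IsHorizontal flag.
; Below that level, the parent behavior runs instead.
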(fn `Call PlayerActionWhenDrilling`
  (params (BPBossRushCharacter :type "/Game/Blueprints/BP_BossRushCharacter Object Reference"))
  (if (>= (`/Game/Blueprints/BP_BossRushCharacter.CurrentDrillLevel` BPBossRushCharacter) (`self.RequiredDrillLevelToBounce`))
    (`/Game/Blueprints/BP_BossRushCharacter.Spawn VFXOn Drill Tip` BPBossRushCharacter "/Game/Art/VFX/Animations/PC_Impact_Walls_VFX.PC_Impact_Walls_VFX" 140.0)
    (bind _newdirectiontodrill (`self.GetNewDrillVector` BPBossRushCharacter))
    (`/Game/Blueprints/BP_BossRushCharacter.DrillIntoADirection` BPBossRushCharacter _newdirectiontodrill)
    (else
      (`parent.Call PlayerActionWhenDrilling` BPBossRushCharacter))))

(fn `GetNewDrillVector`
  (params (Character :type "/Game/Blueprints/BP_BossRushCharacter Object Reference"))
  (returns (NewDirectionToDrill :type "Vector2D Structure"))
  (locals (CharacterAimingDirection :type "Vector2D Structure") (vectorToReturn :type "Vector2D Structure"))
  (bind (_characteraimingdirection_x _characteraimingdirection_y) (`KismetMathLibrary.BreakVector2D` (`local.CharacterAimingDirection`)))
  (set `local.CharacterAimingDirection` (`/Game/Blueprints/BP_BossRushCharacter.AimingDirection` Character))
  (if (`self.isHorizontal`)
    (set `local.vectorToReturn` (`KismetMathLibrary.MakeVector2D` _characteraimingdirection_x (* _characteraimingdirection_y -1.0)))
    (else
      (set `local.vectorToReturn` (`KismetMathLibrary.MakeVector2D` (* _characteraimingdirection_x -1.0) _characteraimingdirection_y))))
  (return (`local.vectorToReturn`)))

(fn `UserConstructionScript`
  (`parent.UserConstructionScript`))
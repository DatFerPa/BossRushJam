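; Kind boss Blueprint for the boss rush game, a child boss that deals contact damage and triggers the player's victory.
; Its Box overlap applies AttackDamage to the player character.
; Any health change event from BP_HealthComponent, with no threshold check here, runs the parent's death handling and has the game mode create the victory menu.
; The same event zeroes player gravity, stops movement and starts the character's victory handling.
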(event `self.Box.OnComponentBeginOverlap`
  (params (OverlappedComponent :type "PrimitiveComponent Object Reference") (OtherActor :type "Actor Object Reference") (OtherComp :type "PrimitiveComponent Object Reference") (OtherBodyIndex :type Integer) (bFromSweep :type Boolean) (SweepResult :type "HitResult Structure (by ref)"))
  (bind _asbp_boss_rush_character (cast `/Game/Blueprints/BP_BossRushCharacter` OtherActor))
  (`GameplayStatics.ApplyDamage` _asbp_boss_rush_character (`self.Attack Damage`)))

(event `self.BP_HealthComponent.OnHealthChanged`
  (params (NewHealth :type "Float (double-precision)"))
  (`self.ManageBossDeath`)
  (bind _asgm_boss_rush_game_mode (cast `/Game/GameConfiguration/GM_BossRushGameMode` (`GameplayStatics.GetGameMode`)))
  (`/Game/GameConfiguration/GM_BossRushGameMode.CreateVictoryMenu` _asgm_boss_rush_game_mode)
  (bind _asbp_boss_rush_character (cast `/Game/Blueprints/BP_BossRushCharacter` (`GameplayStatics.GetPlayerCharacter` 0)))
  (bind _charactermovement (`Character.CharacterMovement` _asbp_boss_rush_character))
  (set `CharacterMovementComponent.GravityScale` 0.0 _charactermovement)
  (`MovementComponent.StopMovementImmediately` _charactermovement)
  (`/Game/Blueprints/BP_BossRushCharacter.ManageCharacterVictory` _asbp_boss_rush_character))

(fn `ManageBossDeath`
  (`parent.ManageBossDeath`))

(fn `UserConstructionScript`
  (`parent.UserConstructionScript`))
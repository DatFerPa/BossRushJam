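; Hand actor for the Scoolio boss that performs front and hammer punches from preset positions near the player, with PaperZD flipbook animation.
; Each punch picks the closest waypoint from its position list, passes that point's left/right flag to the AnimInstance and jumps the punch state machine.
; Separate functions teleport the hand to the selected point, show it, or hide it and park it at a fixed location.
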(event `self.ReceiveBeginPlay`
  (`self.HideHand`)
  (bind _returnvalue (`GameplayStatics.GetActorOfClass` "/Game/Blueprints/Bosses/Scoolio/BP_ScoolioBoss.BP_ScoolioBoss_C"))
  (set `self.Scoolio` _returnvalue)
  (bind _returnvalue_2 (`GameplayStatics.GetActorOfClass` "/Game/Blueprints/BP_BossRushCharacter.BP_BossRushCharacter_C"))
  (set `self.Character` _returnvalue_2))

(fn `Find NearestPoint to Player`
  (params (WayPointsToUse :type "Array of /Game/Blueprints/Bosses/Scoolio/BP_ScoolioWayPoint Object Reference"))
  (locals (CurrentSelectedPosition :type "/Game/Blueprints/Bosses/Scoolio/BP_ScoolioWayPoint Object Reference") (CurrentNearestDistance :type "Float (double-precision)" :default 1000000000000.0))
  (for _array_element WayPointsToUse
    (bind _returnvalue (`KismetMathLibrary.Vector_Distance` (`self.K2_GetActorLocation` (`self.Character`)) (`self.K2_GetActorLocation` _array_element)))
    (if (<= _returnvalue (`local.CurrentNearestDistance`))
      (set `local.CurrentSelectedPosition` _array_element)
      (set `local.CurrentNearestDistance` _returnvalue)))
  (set `self.SelectedPunchPosition` (`local.CurrentSelectedPosition`)))

(fn `HideHand`
  (`SceneComponent.SetVisibility` (`self.PaperFlipbook`) false false)
  (`self.K2_SetActorLocation` (800.0 800.0 800.0) false true))

(fn `PerformFrontPunchOnNearestPositonToPlayer`
  (`self.Find NearestPoint to Player` (`self.FrontPunchPositions`))
  (`self.setLeftHandAttack` (`/Game/Blueprints/Bosses/Scoolio/BP_ScoolioWayPoint.isForLeftHand` (`self.SelectedPunchPosition`)))
  (`PaperZDAnimInstance.JumpToNode` (`PaperZDAnimationComponent.AnimInstance` (`self.PaperZDAnimation`)) "FrontPunch_Jump" "Punch_StateMachine"))

(fn `PerformHammerPunchOnNearesPositionToPlayer`
  (`self.Find NearestPoint to Player` (`self.HammerPunchPositions`))
  (`self.setLeftHandAttack` (`/Game/Blueprints/Bosses/Scoolio/BP_ScoolioWayPoint.isForLeftHand` (`self.SelectedPunchPosition`)))
  (`PaperZDAnimInstance.JumpToNode` (`PaperZDAnimationComponent.AnimInstance` (`self.PaperZDAnimation`)) "HammerPunch_Jump" "Punch_StateMachine"))

(fn `setLeftHandAttack`
  (params (isForLeftHand :type Boolean))
  (bind _aspzdbp_scoolio_hand (cast `/Game/Art/Characters/Scoolio/PZDBP_ScoolioHand` (`PaperZDAnimationComponent.AnimInstance` (`self.PaperZDAnimation`))))
  (set `/Game/Art/Characters/Scoolio/PZDBP_ScoolioHand.isLeft` isForLeftHand _aspzdbp_scoolio_hand))

(fn `ShowHand`
  (`SceneComponent.SetVisibility` (`self.PaperFlipbook`) true false))

(fn `Teleport To Selected Position`
  (`self.K2_SetActorLocation` (`SceneComponent.K2_GetComponentLocation` (`/Game/Blueprints/Bosses/Scoolio/BP_ScoolioWayPoint.DefaultSceneRoot` (`self.SelectedPunchPosition`))) false true))

(fn `UserConstructionScript`)
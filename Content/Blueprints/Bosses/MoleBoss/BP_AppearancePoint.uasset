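; BP_AppearancePoint is an appearance point for the Mole Boss fight, showing an animated dirt effect when activated.
; The flipbook starts hidden, and a reference to the BP_MoleBoss in the level is cached on BeginPlay.
; Activation reveals the flipbook, jumps the PaperZD dirt state machine to its appearing node and flags the point as selected.
; Deactivation jumps to the exiting node and clears the flag, only if the point is selected.
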(event `self.ReceiveBeginPlay`
  (bind _returnvalue (`GameplayStatics.GetActorOfClass` "/Game/Blueprints/Bosses/MoleBoss/BP_MoleBoss.BP_MoleBoss_C"))
  (set `self.MoleBooss` _returnvalue))

(fn `Appear Point Deactivate`
  (if (`self.AppearancePointSelected`)
    (`PaperZDAnimInstance.JumpToNode` (`PaperZDAnimationComponent.AnimInstance` (`self.PaperZDAnimation`)) "Exiting_Jump" "Dirt_StateMachine")
    (set `self.AppearancePointSelected` false)))

(fn `AppearPointActivate`
  (`SceneComponent.SetVisibility` (`self.AppearanceFlipbook`) true false)
  (`PaperZDAnimInstance.JumpToNode` (`PaperZDAnimationComponent.AnimInstance` (`self.PaperZDAnimation`)) "Appearing_Jump" "Dirt_StateMachine")
  (set `self.AppearancePointSelected` true))

(fn `UserConstructionScript`
  (`SceneComponent.SetVisibility` (`self.AppearanceFlipbook`) false false))
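; BP_MovableMap_ is a boss-rush map actor that sinks over time and handles the player's victory over BP_KindBoss.
; On BeginPlay it plays the LS_KindAppear sequence, then, if movable, lowers itself one unit per MoveSpeed delay until it reaches FinalLocation.
; Player overlap with either DestructorDeMundos component fires a one-shot victory that damages the boss, stops movement, swaps boss flipbooks and calls ManageCharacterVictory.
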(event `self.ReceiveBeginPlay`
  (`parent.ReceiveBeginPlay`)
  (bind _outactor (`LevelSequencePlayer.CreateLevelSequencePlayer` "/Game/LevelSequencers/LS_KindAppear.LS_KindAppear" (make `MovieSceneSequencePlaybackSettings` false)))
  (`MovieSceneSequencePlayer.Play` (`LevelSequenceActor.SequencePlayer` _outactor))
  (`KismetSystemLibrary.Delay` 1.0)
  (if (`self.IsMovable`)
    (set `self.RealLocation` (`self.InitialLocation`))
    (`self.MoveMap`)))

(event `MoveMap`
  (if (`self.IsFinalLocation`) :!label _label
    _
    (elif (== (`self.RealLocation`) (`self.FinalLocation`))
      (set `self.IsFinalLocation` true)
      (goto _label)
      (else
        (`KismetSystemLibrary.Delay` (`self.MoveSpeed`))
        (bind _output_get (set `self.RealLocation` (- (`self.RealLocation`) (0.0 0.0 1.0))))
        (`self.K2_SetActorLocation` _output_get)
        (goto _label)))))

(event `self.DestructorDeMundos1.OnComponentBeginOverlap`
  (params (OverlappedComponent :type "PrimitiveComponent Object Reference") (OtherActor :type "Actor Object Reference") (OtherComp :type "PrimitiveComponent Object Reference") (OtherBodyIndex :type Integer) (bFromSweep :type Boolean) (SweepResult :type "HitResult Structure (by ref)"))
  (bind _asbp_boss_rush_character (cast `/Game/Blueprints/BP_BossRushCharacter` OtherActor))
  (`self.ManageVictory` _asbp_boss_rush_character))

(event `self.DestructorDeMundos.OnComponentBeginOverlap`
  (params (OverlappedComponent :type "PrimitiveComponent Object Reference") (OtherActor :type "Actor Object Reference") (OtherComp :type "PrimitiveComponent Object Reference") (OtherBodyIndex :type Integer) (bFromSweep :type Boolean) (SweepResult :type "HitResult Structure (by ref)"))
  (bind _asbp_boss_rush_character (cast `/Game/Blueprints/BP_BossRushCharacter` OtherActor))
  (`self.ManageVictory` _asbp_boss_rush_character))

(event `ManageVictory`
  (params (BP_Character :type "/Game/Blueprints/BP_BossRushCharacter Object Reference"))
  (`/Engine/EditorBlueprintResources/StandardMacros.DoOnce` false
    (:`Completed`
      (bind _returnvalue (`GameplayStatics.GetActorOfClass` "/Game/Blueprints/Bosses/Core_Kind/BP_KindBoss.BP_KindBoss_C"))
      (`GameplayStatics.ApplyDamage` _returnvalue (`self.Attack Damage`))
      (set `self.IsFinalLocation` true)
      (bind _sprite (`PaperCharacter.Sprite` _returnvalue))
      (`PaperFlipbookComponent.SetFlipbook` _sprite "/Game/Art/Ending/Animations/Kind_Spit.Kind_Spit")
      (`KismetSystemLibrary.Delay` 0.4)
      (`PaperFlipbookComponent.SetFlipbook` _sprite "/Game/Art/Ending/Animations/Kind_Spit_NoStick_Flipbook.Kind_Spit_NoStick_Flipbook")
      (`/Game/Blueprints/BP_BossRushCharacter.Manage Character Victory` BP_Character))))

(fn `UserConstructionScript`
  (`parent.UserConstructionScript`))
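; BP_Camera is a camera Blueprint that provides a manually triggered, curve-driven camera shake.
; ManualCameraShake swaps the supplied rotation and location vector curves into a single timeline at runtime, sets its play rate, sizes it to the longer curve and restarts it.
; Each update applies both tracks, scaled by a power multiplier, to the Camera's relative transform, which resets on finish.
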(event `ManualCameraShake`
  (params (RotationCurve :type "CurveVector Object Reference") (LocationCurve :type "CurveVector Object Reference") (PlayRate :type "Float (double-precision)") (PowerMultiplier :type "Float (double-precision)"))
  (set `self.ShakePowerMultiplier` PowerMultiplier)
  (set `self.ShakeRotationCurve` RotationCurve)
  (set `self.ShakeLocationCurve` LocationCurve)
  (`TimelineComponent.SetPlayRate` (`self.CameraShakeTimeline`) PlayRate)
  (`TimelineComponent.SetVectorCurve` (`self.CameraShakeTimeline`) (`self.ShakeRotationCurve`) "Rotation")
  (`TimelineComponent.SetVectorCurve` (`self.CameraShakeTimeline`) (`self.ShakeLocationCurve`) "Location")
  (`TimelineComponent.SetTimelineLength` (`self.CameraShakeTimeline`) (`KismetMathLibrary.FMax` (`.MaxTime` (`CurveBase.GetTimeRange` (`self.ShakeLocationCurve`))) (`.MaxTime` (`CurveBase.GetTimeRange` (`self.ShakeRotationCurve`)))))
  (`TimelineComponent.PlayFromStart` (`self.CameraShakeTimeline`)))

(fn `UserConstructionScript`)
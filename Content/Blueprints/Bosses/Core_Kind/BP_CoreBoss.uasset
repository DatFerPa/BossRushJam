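; BP_CoreBoss is the Core boss's egg stage, which cracks as it takes damage and then hands off to the second-phase level.
; Health component changes play random hurt sounds and step phase flags through three thresholds, each swapping the break flipbook and playing a crack sound.
; At zero health after the last break, it triggers boss death, character victory, camera shake, roar and a hide sequence, then opens 05_Core_Phase2 after a delay.
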(event `self.ReceiveBeginPlay`
  (`parent.ReceiveBeginPlay`)
  (`KismetSystemLibrary.Delay` (`self.DelayBeforeBeatSound`))
  (`PaperZDAnimInstance.JumpToNode` (`PaperZDAnimationComponent.AnimInstance` (`self.AnimationComponent`)) "JumpIdle" "None"))

(event `self.BP_HealthComponent.OnHealthChanged`
  (params (NewHealth :type "Float (double-precision)"))
  (`/Game/Audio/BPFL_Audio.PlayRandom3DSound` (`|MakeArray` "/Game/Audio/Assets/SFX/Characters/EGG/EGG_Damage_1.EGG_Damage_1" "/Game/Audio/Assets/SFX/Characters/EGG/EGG_Damage_2.EGG_Damage_2" "/Game/Audio/Assets/SFX/Characters/EGG/EGG_Damage_3.EGG_Damage_3" :!type "SoundBase Object Reference") "/Game/Audio/MainAttenuation.MainAttenuation" (`self.K2_GetActorLocation`))
  (set `self.CurrentHealth` NewHealth)
  (`|ExecutionSequence`
    (:`then_0`
      (if (`self.IsPhase1`)
        (if (not (>= (`self.CurrentHealth`) (`self.ThresholdPhase1`)))
          (set `self.IsPhase1` false)
          (set `self.IsPhase2` true)
          (`PaperFlipbookComponent.SetFlipbook` (`self.Sprite`) "/Game/Art/Characters/Kind/Animations/Kind_Idle_Break1.Kind_Idle_Break1")
          (`/Game/Audio/BPFL_Audio.PlayRandom3DSound` (`|MakeArray` "/Game/Audio/Assets/SFX/Characters/EGG/EGG_Crack_1.EGG_Crack_1" "/Game/Audio/Assets/SFX/Characters/EGG/EGG_Crack_2.EGG_Crack_2" :!type "SoundBase Object Reference") null (`self.K2_GetActorLocation`) :!label _label))))
    (:`then_1`
      (if (`self.IsPhase2`)
        (if (not (>= (`self.CurrentHealth`) (`self.ThresholdPhase2`)))
          (set `self.IsPhase2` false)
          (set `self.IsPhase3` true)
          (`PaperFlipbookComponent.SetFlipbook` (`self.Sprite`) "/Game/Art/Characters/Kind/Animations/Kind_Idle_Break2.Kind_Idle_Break2")
          (goto _label))))
    (:`then_2`
      (if (`self.IsPhase3`)
        (if (not (>= (`self.CurrentHealth`) (`self.ThresholdPhase3`)))
          (set `self.IsPhase3` false)
          (set `self.ChangeToKind` true)
          (`PaperFlipbookComponent.SetFlipbook` (`self.Sprite`) "/Game/Art/Characters/Kind/Animations/Kind_Idle_Break3.Kind_Idle_Break3")
          (`GameplayStatics.PlaySound2D` "/Game/Audio/Assets/SFX/Characters/EGG/EGG_Crack_3.EGG_Crack_3" 1.0 1.0 0.0 null null))))
    (:`then_3`
      (if (`self.ChangeToKind`)
        (if (== (`self.CurrentHealth`) 0.0)
          (`self.ManageBossDeath`)
          (bind _returnvalue (`GameplayStatics.GetActorOfClass` "/Game/Blueprints/BP_BossRushCharacter.BP_BossRushCharacter_C"))
          (`/Game/Blueprints/BP_BossRushCharacter.Manage Character Victory` _returnvalue)
          (`/Game/Blueprints/Camera/BP_Camera.ManualCameraShake` (`/Game/GameConfiguration/GM_BossRushGameMode.BP_Camera` (cast `/Game/GameConfiguration/GM_BossRushGameMode` (`GameplayStatics.GetGameMode`) :!pure true)) "/Game/Blueprints/Camera/CameraShakeCurve_CoreRotation.CameraShakeCurve_CoreRotation" "/Game/Blueprints/Camera/CameraShakeCurve_CoreLocation.CameraShakeCurve_CoreLocation" 1.0 0.3)
          (`GameplayStatics.PlaySound2D` "/Game/Audio/Assets/SFX/Characters/EGG/EGG_RumbleRoar.EGG_RumbleRoar" 1.0 1.0 0.0 null null)
          (bind _outactor (`LevelSequencePlayer.CreateLevelSequencePlayer` "/Game/LevelSequencers/LS_CoreHide.LS_CoreHide" (make `MovieSceneSequencePlaybackSettings` false)))
          (`MovieSceneSequencePlayer.Play` (`LevelSequenceActor.SequencePlayer` _outactor))
          (`KismetSystemLibrary.Delay` 6.0)
          (`GameplayStatics.OpenLevelBySoftObjectPtr` "/Game/Maps/BossRushGameLevels/05_Core_Phase2.05_Core_Phase2"))))))

(fn `UserConstructionScript`
  (`parent.UserConstructionScript`))
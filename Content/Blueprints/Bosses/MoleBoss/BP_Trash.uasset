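; Trash projectile for the Mole boss that damages the boss-rush player on overlap, unless they are drilling or immune.
; Construction picks a random flipbook and Y offset; StartMovement selects one of five timeline trajectories, mirrored on X by IsLeft.
; Hitting player or map plays destruction flipbook and sound, disables collision, leaves the GameMode's projectile list, notifies MoleBoss and hides the sprite.
; A lifespan timer destroys the actor.
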(event `self.SphereCollision.OnComponentBeginOverlap`
  (params (OverlappedComponent :type "PrimitiveComponent Object Reference") (OtherActor :type "Actor Object Reference") (OtherComp :type "PrimitiveComponent Object Reference") (OtherBodyIndex :type Integer) (bFromSweep :type Boolean) (SweepResult :type "HitResult Structure (by ref)"))
  (bind _paperflipbook (`self.PaperFlipbook`))
  (cast `/Game/Blueprints/BP_BossRushCharacter` OtherActor
    (:`then`
      _)
    (:`CastFailed`
      (cast `/Game/Blueprints/Map/BP_BasicMap` OtherActor)))
  (`PaperFlipbookComponent.SetFlipbook` _paperflipbook (`|GetArrayItem` (`self.DestroyPaperFlipbooks`) (`self.UsedTrash`)))
  (`PaperFlipbookComponent.PlayFromStart` _paperflipbook)
  (`/Game/Audio/BPFL_Audio.PlayRandom3DSound` (`|MakeArray` "/Game/Audio/Assets/SFX/Characters/Molenius/Mol_Trash_Destroy_1.Mol_Trash_Destroy_1" "/Game/Audio/Assets/SFX/Characters/Molenius/Mol_Trash_Destroy_2.Mol_Trash_Destroy_2" "/Game/Audio/Assets/SFX/Characters/Molenius/Mol_Trash_Destroy_3.Mol_Trash_Destroy_3" :!type "SoundBase Object Reference") "/Game/Audio/MainAttenuation.MainAttenuation" (`self.K2_GetActorLocation`))
  (`self.CollisionBehaviour` OtherActor)
  (`KismetSystemLibrary.Delay` 0.2)
  (`SceneComponent.SetVisibility` (`self.PaperFlipbook`) false false))

(event `self.ReceiveBeginPlay`
  (`KismetSystemLibrary.K2_SetTimerDelegate` (delegate `Delete`) (`self.lifespan`))
  (bind _asgm_boss_rush_game_mode (cast `/Game/GameConfiguration/GM_BossRushGameMode` (`GameplayStatics.GetGameMode`)))
  (`KismetArrayLibrary.Array_Add` (`/Game/GameConfiguration/GM_BossRushGameMode.Projectiles` _asgm_boss_rush_game_mode) self))

(event `Delete`
  (`self.K2_DestroyActor`))

(event `StartMovement`
  (params (TrashTrajectory :type Integer))
  (switch `int` TrashTrajectory
    (:`Default`
      (bind (_direction _trashtrack_5) (`Timeline|TrashTimeline_5` :!via `PlayFromStart` :!label _label)
        (:`Update`
          (`self.MoveTrash` _trashtrack_5))))
    (:`0`
      (bind (_direction_2 _trashtrack_1) (`Timeline|TrashMovementTimeline_1` :!via `PlayFromStart`)
        (:`Update`
          (`self.MoveTrash` _trashtrack_1))))
    (:`1`
      (bind (_direction_3 _trashtrack_2) (`Timeline|TrashTimeline_2` :!via `PlayFromStart`)
        (:`Update`
          (`self.MoveTrash` _trashtrack_2))))
    (:`2`
      (bind (_direction_4 _trashtrack_3) (`Timeline|TrashTimeline_3` :!via `PlayFromStart`)
        (:`Update`
          (`self.MoveTrash` _trashtrack_3))))
    (:`3`
      (bind (_direction_5 _trashtrack_4) (`Timeline|TrashTimeline_4` :!via `PlayFromStart`)
        (:`Update`
          (`self.MoveTrash` _trashtrack_4))))
    (:`4`
      (goto _label :!via `PlayFromStart`))))

(fn `CollisionBehaviour`
  (params (Actor :type "Actor Object Reference"))
  (bind _asbp_boss_rush_character (cast `/Game/Blueprints/BP_BossRushCharacter` Actor)
    (:`then`
      (if (or (`/Game/Blueprints/BP_BossRushCharacter.isDrilling` _asbp_boss_rush_character) (`/Game/Blueprints/BP_BossRushCharacter.isInmune` _asbp_boss_rush_character))
        (`/Game/Blueprints/BP_BossRushCharacter.Spawn VFX` :`self` _asbp_boss_rush_character :`FlipbookToUse` "/Game/Art/VFX/Animations/PC_Impact_Walls_VFX.PC_Impact_Walls_VFX" :`SpawnLocation` (`SceneComponent.K2_GetComponentLocation` (`/Game/Blueprints/BP_BossRushCharacter.CenterCharacter` _asbp_boss_rush_character)))
        (else
          (`GameplayStatics.ApplyDamage` _asbp_boss_rush_character (`self.Damage`)))))
    (:`CastFailed`
      (cast `/Game/Blueprints/Map/BP_BasicMap` Actor)))
  (`self.DeleteTheTrash`))

(fn `DeleteTheTrash`
  (`PrimitiveComponent.SetCollisionEnabled` (`self.SphereCollision`) "NoCollision")
  (bind _asgm_boss_rush_game_mode (cast `/Game/GameConfiguration/GM_BossRushGameMode` (`GameplayStatics.GetGameMode`)))
  (`KismetArrayLibrary.Array_RemoveItem` (`/Game/GameConfiguration/GM_BossRushGameMode.Projectiles` _asgm_boss_rush_game_mode) self)
  (`/Game/Blueprints/Bosses/MoleBoss/BP_MoleBoss.TrashDestroyed` (`self.MoleBoss`)))

(fn `GenerateRandomFlipbook`
  (bind _paperflibookstouse (`self.PaperFlibooksToUse`))
  (bind _output_get (set `self.UsedTrash` (`KismetMathLibrary.RandomIntegerInRange` 0 (- (`KismetArrayLibrary.Array_Length` _paperflibookstouse) 1))))
  (`PaperFlipbookComponent.SetFlipbook` (`self.PaperFlipbook`) (`|GetArrayItem` _paperflibookstouse _output_get)))

(fn `MoveTrash`
  (params (MovementVector :type "Vector Structure"))
  (if (`self.isLeft`)
    (`self.K2_SetActorRelativeLocation` (`KismetMathLibrary.MakeVector` (* MovementVector_X -1.0) 0.0 MovementVector_Z))
    (else
      (`self.K2_SetActorRelativeLocation` (`KismetMathLibrary.MakeVector` MovementVector_X 0.0 MovementVector_Z)))))

(fn `RandomYPosition`
  (`SceneComponent.K2_SetRelativeLocation` (`self.PaperFlipbook`) (`KismetMathLibrary.MakeVector` 0.0 (`KismetMathLibrary.RandomFloatInRange` -5.0 5.0)) false true))

(fn `UserConstructionScript`
  (`self.GenerateRandomFlipbook`)
  (`self.RandomYPosition`))
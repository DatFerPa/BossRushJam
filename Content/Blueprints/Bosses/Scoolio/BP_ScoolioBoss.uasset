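; Boss-rush boss Scoolio, with horns, eyes and a separate BP_ScoolioHand actor that joins its hit blink.
; It glides between random waypoints on a timeline or teleports to appear, hammer-head attack at the point nearest the player, and die.
; Animation state machine jumps play those actions, with bone VFX for head smashes.
; Health changes feed the blackboard, and death switches head collision to WorldStatic before running parent death handling.
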(event `self.ReceiveBeginPlay`
  (bind _scooliohand (`self.ScoolioHand`))
  (bind _bossspritestohitblink (`self.BossSpritesToHitBlink`))
  (`parent.ReceiveBeginPlay`)
  (`|ExecutionSequence`
    (:`then_0`
      (`KismetArrayLibrary.Array_Add` _bossspritestohitblink (`self.Eye_Right`))
      (`KismetArrayLibrary.Array_Add` _bossspritestohitblink (`self.Eye_Left`))
      (`KismetArrayLibrary.Array_Add` _bossspritestohitblink (`self.Horns`))
      (bind _returnvalue (`GameplayStatics.GetActorOfClass` "/Game/Blueprints/Bosses/Scoolio/BP_ScoolioHand.BP_ScoolioHand_C"))
      (bind _output_get (set `self.ScoolioHand` _returnvalue))
      (`/Engine/EditorBlueprintResources/StandardMacros.IsValid` _output_get
        (:`Is Valid`
          (`KismetArrayLibrary.Array_Add` _bossspritestohitblink (`/Game/Blueprints/Bosses/Scoolio/BP_ScoolioHand.PaperFlipbook` _scooliohand))
          (bind _asgm_boss_rush_game_mode (cast `/Game/GameConfiguration/GM_BossRushGameMode` (`GameplayStatics.GetGameMode`)))
          (`KismetArrayLibrary.Array_Add` (`/Game/GameConfiguration/GM_BossRushGameMode.Projectiles` _asgm_boss_rush_game_mode) _scooliohand))))
    (:`then_1`
      (bind _aspzdbp_scoolio_eyes (cast `/Game/Art/Characters/Scoolio/PZDBP_ScoolioEyes` (`PaperZDAnimationComponent.AnimInstance` (`self.EyeLeft_AnimationComponent`))))
      (set `/Game/Art/Characters/Scoolio/PZDBP_ScoolioEyes.isLeft` true _aspzdbp_scoolio_eyes))
    (:`then_2`
      (bind _returnvalue_2 (`GameplayStatics.GetActorOfClass` "/Game/Blueprints/BP_BossRushCharacter.BP_BossRushCharacter_C"))
      (set `self.Character` _returnvalue_2)
      (`self.UpdateBlackboardHealthValue` (`/Game/Blueprints/Components/BP_HealthComponent.MaxHealth` (`self.BP_HealthComponent`))))))

(event `MoveScoolioToWayPoint`
  (`self.SelectRandomWayPointToMove`)
  (set `self.StartingLocation` (`self.K2_GetActorLocation`))
  (bind (_direction _movementpercentaje) (`Timeline|ScoolioMovementTimeline` :!via `PlayFromStart`)
    (:`Update`
      (`self.K2_SetActorLocation` (`KismetMathLibrary.VLerp` (`self.StartingLocation`) (`self.K2_GetActorLocation` (`self.SelectedWayPointToMove`)) _movementpercentaje)))
    (:`Finished`
      (`self.FinishAttack`))))

(event `self.BP_HealthComponent.OnHealthChanged`
  (params (NewHealth :type "Float (double-precision)"))
  (`self.UpdateBlackboardHealthValue` NewHealth))

(event `self.BP_HealthComponent.OnDeath`
  (`self.ManageBossDeath`))

(fn `HammerHeadAttack`
  (`self.SelectNearThePlayerWayPoint` (`self.HammerAttacksLocation`))
  (`PaperZDAnimInstance.JumpToNode` (`PaperZDAnimationComponent.AnimInstance` (`self.AnimationComponent`)) "HeadAttack_Jump" "Scoolio_StateMachine")
  (`self.K2_SetActorLocation` (`SceneComponent.K2_GetComponentLocation` (`/Game/Blueprints/Bosses/Scoolio/BP_ScoolioWayPoint.DefaultSceneRoot` (`self.SelectedWayPointToMove`))) false true))

(fn `HideScoolio`
  (`self.K2_SetActorLocation` (500.0 500.0 500.0) false true))

(fn `ManageBossDeath`
  (`PrimitiveComponent.SetCollisionObjectType` (`self.HeadCollisionToDamage`) "ECC_WorldStatic")
  (`parent.ManageBossDeath`))

(fn `ScoolioAppears`
  (`self.TeleportScoolioToRandomWayPoint`)
  (`PaperZDAnimInstance.JumpToNode` (`PaperZDAnimationComponent.AnimInstance` (`self.AnimationComponent`)) "Appear_Jump" "Scoolio_StateMachine"))

(fn `ScoolioDies`
  (bind _hammerattackslocation (`self.HammerAttacksLocation`))
  (bind _output_get (set `self.SelectedWayPointToMove` (`|GetArrayItem` _hammerattackslocation (`KismetMathLibrary.RandomInteger` (`KismetArrayLibrary.Array_Length` _hammerattackslocation)))))
  (`self.K2_SetActorLocation` (`self.K2_GetActorLocation` _output_get) false true)
  (`PaperZDAnimInstance.JumpToNode` (`PaperZDAnimationComponent.AnimInstance` (`self.AnimationComponent`)) "Dying_Jump" "Scoolio_StateMachine"))

(fn `ScoolioDissapears`
  (`PaperZDAnimInstance.JumpToNode` (`PaperZDAnimationComponent.AnimInstance` (`self.AnimationComponent`)) "Dissappear_Jump" "Scoolio_StateMachine"))

(fn `ScoolioVisibility`
  (params (HornsAndEyesVisibility :type Boolean) (BodyVisibility :type Boolean))
  (`SceneComponent.SetVisibility` (`self.Scoolio_Visual`) HornsAndEyesVisibility true)
  (`SceneComponent.SetVisibility` (`self.Sprite`) BodyVisibility false))

(fn `SelectNearThePlayerWayPoint`
  (params (WayPointsToUse :type "Array of /Game/Blueprints/Bosses/Scoolio/BP_ScoolioWayPoint Object Reference"))
  (locals (CurrentSelectedPosition :type "/Game/Blueprints/Bosses/Scoolio/BP_ScoolioWayPoint Object Reference") (CurrentNearestPosition :type "Float (double-precision)" :default 10000000000.0))
  (for _array_element WayPointsToUse
    (bind _returnvalue (`KismetMathLibrary.Vector_Distance` (`self.K2_GetActorLocation` (`self.Character`)) (`self.K2_GetActorLocation` _array_element)))
    (if (<= _returnvalue (`local.CurrentNearestPosition`))
      (set `local.CurrentSelectedPosition` _array_element)
      (set `local.CurrentNearestPosition` _returnvalue)))
  (set `self.SelectedWayPointToMove` (`local.CurrentSelectedPosition`)))

(fn `SelectRandomWayPointToMove`
  (bind _waypoints (`self.WayPoints`))
  (set `self.SelectedWayPointToMove` (`|GetArrayItem` _waypoints (`KismetMathLibrary.RandomInteger` (`KismetArrayLibrary.Array_Length` _waypoints)))))

(fn `SpawnVFXWhenHeadSmash`
  (`|SpawnActorFromClass` "/Game/Blueprints/Actors_VFX/BP_BasicImpactVFX.BP_BasicImpactVFX_C" (`KismetMathLibrary.MakeTransform` (`SceneComponent.K2_GetComponentLocation` (`self.VFX_HeadSmash_Right`))) "Undefined" "MultiplyWithRoot" null "/Game/Art/VFX/Animations/Scoolio_BonesA_VFX.Scoolio_BonesA_VFX" 140.0 null)
  (`|SpawnActorFromClass` "/Game/Blueprints/Actors_VFX/BP_BasicImpactVFX.BP_BasicImpactVFX_C" (`KismetMathLibrary.MakeTransform` (`SceneComponent.K2_GetComponentLocation` (`self.VFX_HeadSmash_Left`))) "Undefined" "MultiplyWithRoot" null "/Game/Art/VFX/Animations/Scoolio_BonesB_VFX.Scoolio_BonesB_VFX" 140.0 null))

(fn `TeleportScoolioToRandomWayPoint`
  (`self.SelectRandomWayPointToMove`)
  (`self.K2_SetActorLocation` (`self.K2_GetActorLocation` (`self.SelectedWayPointToMove`)) false true))

(fn `UserConstructionScript`
  (`parent.UserConstructionScript`)
  (set `self.SpriteMaterial` "/Game/Art/materials/MT_ScoolioWindEffect.MT_ScoolioWindEffect"))
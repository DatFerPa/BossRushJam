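; Projectile for the DiamondHead boss that damages the player on contact, using a PaperZD animation instance for its visuals.
; A box overlap with the map or the player stops movement and jumps to the splinter animation, dealing damage only to a non-immune player.
; A timer started at BeginPlay destroys the actor.
; Logic to launch it toward the player along a timeline speed curve is present but unconnected.
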(event `self.ReceiveBeginPlay`
  ;[1 1 1] Begin Play
  (`KismetSystemLibrary.K2_SetTimer` null "DestructionOutOfCamera" (`self.TimeBeforeSelfDestruction`))
  (set `self.ABP` (`PaperZDAnimationComponent.AnimInstance` (`self.PaperZDAnimation`))))

(event `self.Box.OnComponentBeginOverlap`
  (params (OverlappedComponent :type "PrimitiveComponent Object Reference") (OtherActor :type "Actor Object Reference") (OtherComp :type "PrimitiveComponent Object Reference") (OtherBodyIndex :type Integer) (bFromSweep :type Boolean) (SweepResult :type "HitResult Structure (by ref)"))
  (bind _playercharacter (`self.PlayerCharacter`))
  ;[1 1 1] On Begin Overlap
  (cast `/Game/Blueprints/Map/BP_BasicMap` OtherActor
    (:`then`
      (`self.DestructionInCamera`))
    (:`CastFailed`
      (if (== OtherActor _playercharacter)
        (if (not (`/Game/Blueprints/BP_BossRushCharacter.isInmune` _playercharacter))
          (`GameplayStatics.ApplyDamage` (`self.PlayerCharacter`) (`self.ProjectileDamage`))
          (`self.DestructionInCamera`)
          (else
            (`self.DestructionInCamera`)))))))

(fn `DestructionInCamera`
  (`PaperZDAnimInstance.JumpToNode` (`self.ABP`) "JumpSplinter" "None")
  (set `MovementComponent.Velocity` (0.0 0.0 0.0) (`self.ProjectileMovement`)))

(fn `DestructionOutOfCamera`
  (`self.K2_DestroyActor`))

(fn `UserConstructionScript`)